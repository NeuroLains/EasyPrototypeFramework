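; BPC_Attributes is an RPG component that manages an owner's attributes and spendable attribute points, seeded from a data table row unless a save was loaded.
; Point changes, per-level gains, resets and flat or percentage bonuses recalculate final values.
; Each final-value difference adds or removes scaled bonuses on BPC_Stats, updates registered widgets and fires change events.
; State saves to the GameInstance or a save slot; debug mode checks table consistency.
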(event `Initialize`
  (set `self.StatsComponent` (`Actor.GetComponentByClass` (`self.GetOwner`) "/Game/O_RPG/OpenRPG_Stats/Blueprints/Components/BPC_Stats.BPC_Stats_C"))
  (if (`self.DebugEnabled?`)
    (`self.CheckConsistency`))
  (if (not (`self.HasLoadBeenSuccessful?`))
    (`self.LoadTableData`))
  (`self.RefreshWidgets`))

(event `UpdateAttributePoints`
  (params (AvailablePoints :type Integer))
  ;[1 0.1647 0.1349] Attributes and Stats
  (for _array_element (`self.Widgets`)
    (message `/Game/O_RPG/OpenRPG_Stats/Blueprints/Interfaces/BPI_Attributes.UpdateDisplayedAttributePoints` _array_element AvailablePoints)))

(event `UpdateAttributeValue`
  (params (Attribute :type "/Game/O_RPG/OpenRPG_Stats/Enums/e_Attribute Enum" :default "NewEnumerator6") (NewValue :type Integer))
  ;[1 0.1647 0.1349] Attributes and Stats
  (for _array_element (`self.Widgets`)
    (message `/Game/O_RPG/OpenRPG_Stats/Blueprints/Interfaces/BPI_Attributes.UpdateDisplayedAttribute` _array_element Attribute NewValue)))

(fn `AddAttributeBonuses`
  (params (AttributeBonuses :type "/Game/O_RPG/OpenRPG_Stats/Structs/s_AttributeBonus Structure"))
  (locals (LocalFlatBonuses :type "Map of /Game/O_RPG/OpenRPG_Stats/Enums/e_Attribute Enum to Float (double-precision)") (LocalPercentageBonuses :type "Map of /Game/O_RPG/OpenRPG_Stats/Enums/e_Attribute Enum to Float (double-precision)") (LocalCurrentLoopAttribute :type "/Game/O_RPG/OpenRPG_Stats/Enums/e_Attribute Enum") (LocalCurrentLoopAttributeData :type "/Game/O_RPG/OpenRPG_Stats/Structs/s_Attribute Structure") (LocalModifiedAttributes :type "Array of /Game/O_RPG/OpenRPG_Stats/Enums/e_Attribute Enum"))
  (bind (_flatbonuses _percentagebonuses) (break `/Game/O_RPG/OpenRPG_Stats/Structs/s_AttributeBonus` AttributeBonuses))
  (set `local.LocalFlatBonuses` _flatbonuses)
  (set `local.LocalPercentageBonuses` _percentagebonuses)
  (bind _keys (`BlueprintMapLibrary.Map_Keys` (`local.LocalFlatBonuses`)))
  (bind _output_get (set `local.LocalModifiedAttributes` _keys))
  (for _array_element _output_get
    (bind _output_get_2 (set `local.LocalCurrentLoopAttribute` _array_element))
    (bind _output_get_3 (set `local.LocalCurrentLoopAttributeData` (`BlueprintMapLibrary.Map_Find` (`self.Attributes`) _output_get_2)))
    (bind _structout (setmembers `/Game/O_RPG/OpenRPG_Stats/Structs/s_Attribute` :`StructRef` _output_get_3 :`FlatBonuses` (+ (`.FlatBonuses_28_3F6008684D9845B3258C57AB96242FE5` (break `/Game/O_RPG/OpenRPG_Stats/Structs/s_Attribute` _output_get_3)) (`BlueprintMapLibrary.Map_Find` (`local.LocalFlatBonuses`) (`local.LocalCurrentLoopAttribute`)))))
    (`BlueprintMapLibrary.Map_Add` (`self.Attributes`) (`local.LocalCurrentLoopAttribute`) _structout))
  (bind _keys_2 (`BlueprintMapLibrary.Map_Keys` (`local.LocalPercentageBonuses`)))
  (for _array_element_2 _keys_2
    (bind _output_get_4 (set `local.LocalCurrentLoopAttribute` _array_element_2))
    (bind _output_get_5 (set `local.LocalCurrentLoopAttributeData` (`BlueprintMapLibrary.Map_Find` (`self.Attributes`) _output_get_4)))
    (bind _structout_2 (setmembers `/Game/O_RPG/OpenRPG_Stats/Structs/s_Attribute` :`StructRef` _output_get_5 :`PercentageBonuses` (+ (`.PercentageBonuses_29_4A36E47747DB8544BA56E4AF979B4155` (break `/Game/O_RPG/OpenRPG_Stats/Structs/s_Attribute` _output_get_5)) (`BlueprintMapLibrary.Map_Find` (`local.LocalPercentageBonuses`) (`local.LocalCurrentLoopAttribute`)))))
    (`BlueprintMapLibrary.Map_Add` (`self.Attributes`) (`local.LocalCurrentLoopAttribute`) _structout_2)
    (`KismetArrayLibrary.Array_AddUnique` (`local.LocalModifiedAttributes`) (`local.LocalCurrentLoopAttribute`)))
  (`self.CalculateAttributesFinalValues` (`local.LocalModifiedAttributes`))
  (return))

(fn `AddAttributeBonusesToStats`
  (params (Attribute :type "/Game/O_RPG/OpenRPG_Stats/Enums/e_Attribute Enum" :default "NewEnumerator6") (ReceivedPoints :type Integer))
  (locals (LocalAttribute :type "/Game/O_RPG/OpenRPG_Stats/Enums/e_Attribute Enum" :default "NewEnumerator6") (LocalPoints :type Integer) (LocalStatBonuses :type "/Game/O_RPG/OpenRPG_Stats/Structs/s_StatBonus Structure") (`LocalRemove?` :type Boolean))
  (bind (_value _returnvalue) (`BlueprintMapLibrary.Map_Find` (`.AttributeBonusesToStats_10_623131B64D373095975842BC34C25A8D` (break `/Game/O_RPG/OpenRPG_Stats/Structs/s_AttributesData` (`self.GetAttributesData`))) (`local.LocalAttribute`)))
  (set `local.LocalAttribute` Attribute)
  (bind _output_get (set `local.LocalPoints` ReceivedPoints))
  (`/Engine/EditorBlueprintResources/StandardMacros.CompareInt` _output_get
    (:`>`
      _)
    (:`==`
      (return))
    (:`<`
      (set `local.LocalRemove?` true)
      (set `local.LocalPoints` (`KismetMathLibrary.Abs_Int` (`local.LocalPoints`)))))
  (if _returnvalue
    (set `local.LocalStatBonuses` _value)
    (if (`local.LocalRemove?`)
      (`/Game/O_RPG/OpenRPG_Stats/Blueprints/Components/BPC_Stats.RemoveStatBonuses` (`self.StatsComponent`) (`local.LocalStatBonuses`) (`local.LocalPoints`))
      (return)
      (else
        (`/Game/O_RPG/OpenRPG_Stats/Blueprints/Components/BPC_Stats.AddStatBonuses` (`self.StatsComponent`) (`local.LocalStatBonuses`) (`local.LocalPoints`))
        (return)))
    (else
      (return))))

(fn `AddAttributesPerLevel`
  (locals (LocalCurrentLoopAttribute :type "/Game/O_RPG/OpenRPG_Stats/Enums/e_Attribute Enum") (LocalAttributesPerLevel :type "Map of /Game/O_RPG/OpenRPG_Stats/Enums/e_Attribute Enum to Object Object Reference"))
  (bind _output_get (set `local.LocalAttributesPerLevel` (`.AttributesPerLevel_15_EE2E70BF41ED7F6EF3231CBA9014991C` (break `/Game/O_RPG/OpenRPG_Stats/Structs/s_AttributesData` (`self.GetAttributesData`)))))
  (bind _keys (`BlueprintMapLibrary.Map_Keys` _output_get))
  (for _array_element _keys
    (bind _output_get_2 (set `local.LocalCurrentLoopAttribute` _array_element))
    (`self.AddPointsToAttribute` (`local.LocalCurrentLoopAttribute`) (`BlueprintMapLibrary.Map_Find` (`local.LocalAttributesPerLevel`) _output_get_2)))
  (return))

(fn `AddCustomWidgets`
  (params (Widgets :type "Array of UserWidget Object Reference"))
  (for _array_element Widgets
    (`KismetArrayLibrary.Array_AddUnique` (`self.Widgets`) _array_element))
  (return))

(fn `AddPointsToAttribute`
  (params (Attribute :type "/Game/O_RPG/OpenRPG_Stats/Enums/e_Attribute Enum" :default "NewEnumerator6") (Points :type Integer))
  (locals (LocalAttribute :type "/Game/O_RPG/OpenRPG_Stats/Enums/e_Attribute Enum") (LocalPoints :type Integer) (LocalAttributeData :type "/Game/O_RPG/OpenRPG_Stats/Structs/s_Attribute Structure"))
  (bind (_value _returnvalue) (`BlueprintMapLibrary.Map_Find` (`self.Attributes`) (`local.LocalAttribute`)))
  (set `local.LocalAttribute` Attribute)
  (bind _output_get (set `local.LocalPoints` Points))
  (if (!= _output_get 0)
    (if _returnvalue
      (bind _output_get_2 (set `local.LocalAttributeData` _value))
      (bind _structout (setmembers `/Game/O_RPG/OpenRPG_Stats/Structs/s_Attribute` :`StructRef` _output_get_2 :`BaseValue` (+ (`.BaseValue_5_5398D8464682C14444DF888899E8366F` (break `/Game/O_RPG/OpenRPG_Stats/Structs/s_Attribute` _output_get_2)) (`local.LocalPoints`))))
      (`BlueprintMapLibrary.Map_Add` (`self.Attributes`) (`local.LocalAttribute`) _structout)
      (`self.CalculateAttributesFinalValues` (`|MakeArray` (`local.LocalAttribute`)))
      (return)
      (else
        (return)))
    (else
      (return))))

(fn `CalculateAttributesFinalValues`
  (params (ModifiedAttributes :type "Array of /Game/O_RPG/OpenRPG_Stats/Enums/e_Attribute Enum"))
  (locals (LocalCurrentLoopAttribute :type "/Game/O_RPG/OpenRPG_Stats/Enums/e_Attribute Enum") (LocalCurrentLoopAttributeData :type "/Game/O_RPG/OpenRPG_Stats/Structs/s_Attribute Structure") (LocalPreviousValue :type Integer) (LocalPreviousAttributeValues :type "Map of /Game/O_RPG/OpenRPG_Stats/Enums/e_Attribute Enum to Integer") (LocalPointsDifference :type Integer :default 0) (LocalModifiedAttributes :type "Array of /Game/O_RPG/OpenRPG_Stats/Enums/e_Attribute Enum"))
  (bind _localcurrentloopattribute (`local.LocalCurrentLoopAttribute`))
  (bind _localcurrentloopattribute_2 (`local.LocalCurrentLoopAttribute`))
  (bind _output_get (set `local.LocalModifiedAttributes` ModifiedAttributes))
  (for _array_element _output_get
    (`BlueprintMapLibrary.Map_Add` (`local.LocalPreviousAttributeValues`) _array_element (`self.GetAttributeValue` _array_element)))
  (for _array_element_2 (`local.LocalModifiedAttributes`)
    (bind _output_get_2 (set `local.LocalCurrentLoopAttribute` _array_element_2))
    (bind _output_get_3 (set `local.LocalCurrentLoopAttributeData` (`BlueprintMapLibrary.Map_Find` (`self.Attributes`) _output_get_2)))
    (bind (_basevalue _flatbonuses _percentagebonuses _finalvalue) (break `/Game/O_RPG/OpenRPG_Stats/Structs/s_Attribute` _output_get_3))
    (set `local.LocalPreviousValue` _finalvalue)
    (bind _structout (setmembers `/Game/O_RPG/OpenRPG_Stats/Structs/s_Attribute` :`StructRef` _output_get_3 :`FinalValue` (+ _basevalue (`KismetMathLibrary.FTrunc` _flatbonuses) (`KismetMathLibrary.FTrunc` (/ (* _basevalue _percentagebonuses) 100.0)))))
    (`BlueprintMapLibrary.Map_Add` (`self.Attributes`) (`local.LocalCurrentLoopAttribute`) _structout)
    (bind _output_get_4 (set `local.LocalPointsDifference` (- (`self.GetAttributeValue` (`local.LocalCurrentLoopAttribute`)) (`BlueprintMapLibrary.Map_Find` (`local.LocalPreviousAttributeValues`) (`local.LocalCurrentLoopAttribute`)))))
    (if (!= _output_get_4 0)
      (`self.AddAttributeBonusesToStats` (`local.LocalCurrentLoopAttribute`) (`local.LocalPointsDifference`))
      (`self.UpdateAttributeValue` _localcurrentloopattribute (`self.GetAttributeValue` _localcurrentloopattribute))
      (`self.OnAttributeFinalValueChanged` _localcurrentloopattribute_2 (`local.LocalPreviousValue`) (`self.GetAttributeValue` _localcurrentloopattribute_2))))
  (return))

(fn `CheckConsistency`
  (locals (LocalDefaultAttributes :type "/Game/O_RPG/OpenRPG_Stats/Structs/s_AttributesData Structure") (LocalAttribute :type "/Game/O_RPG/OpenRPG_Stats/Enums/e_Attribute Enum"))
  (`/Engine/EditorBlueprintResources/StandardMacros.IsValid` (`self.AttributesTable`)
    (:`Is Valid`
      (bind _returnvalue (`|GetDataTableRow` (`self.AttributesTable`) (`self.AttributesTableRow`))
        (:`then`
          (bind _output_get (set `local.LocalDefaultAttributes` _returnvalue))
          (bind _keys (`BlueprintMapLibrary.Map_Keys` (`.AttributeBonusesToStats_10_623131B64D373095975842BC34C25A8D` (break `/Game/O_RPG/OpenRPG_Stats/Structs/s_AttributesData` _output_get))))
          (for _array_element _keys
            (bind _output_get_2 (set `local.LocalAttribute` _array_element))
            (if (not (`BlueprintMapLibrary.Map_Contains` (`.Attributes_16_BA76E1204E2CD013510F85AB363740DC` (break `/Game/O_RPG/OpenRPG_Stats/Structs/s_AttributesData` (`local.LocalDefaultAttributes`))) _output_get_2))
              (`KismetSystemLibrary.PrintString` (`KismetStringLibrary.Concat_StrStr` "Warning: Attribute " (`|GetEnumeratorNameAsString` (`local.LocalAttribute`)) " found in AttributeBonusesToStats but not in Attributes, clean that data!") true false (struct :`R` 1.0 :`G` 1.0 :`A` 1.0) 10.0)))
          (bind _keys_2 (`BlueprintMapLibrary.Map_Keys` (`.AttributesPerLevel_15_EE2E70BF41ED7F6EF3231CBA9014991C` (break `/Game/O_RPG/OpenRPG_Stats/Structs/s_AttributesData` (`local.LocalDefaultAttributes`)))))
          (for _array_element_2 _keys_2
            (bind _output_get_3 (set `local.LocalAttribute` _array_element_2))
            (if (not (`BlueprintMapLibrary.Map_Contains` (`.Attributes_16_BA76E1204E2CD013510F85AB363740DC` (break `/Game/O_RPG/OpenRPG_Stats/Structs/s_AttributesData` (`local.LocalDefaultAttributes`))) _output_get_3))
              (`KismetSystemLibrary.PrintString` (`KismetStringLibrary.Concat_StrStr` "Warning: Attribute " (`|GetEnumeratorNameAsString` (`local.LocalAttribute`)) " found in AttributesPerLevel but not in Attributes, clean that data!") true false (struct :`R` 1.0 :`G` 1.0 :`A` 1.0) 10.0)))
          (`KismetSystemLibrary.PrintString` "No errors found!" true false (struct :`G` 1.0 :`A` 1.0) 5.0)
          (return))
        (:`RowNotFound`
          (`KismetSystemLibrary.PrintString` (`KismetStringLibrary.Concat_StrStr` "AttributesTableRow " (`KismetStringLibrary.Conv_NameToString` (`self.AttributesTableRow`)) " not found in AttributesTable") true false (struct :`R` 1.0 :`A` 1.0) 10.0)
          (return))))
    (:`Is Not Valid`
      (`KismetSystemLibrary.PrintString` "Error: Not valid AttributesTable value assigned" true false (struct :`R` 1.0 :`A` 1.0) 10.0)
      (return))))

(fn `CreateSaveData`
  (returns (Data :type "/Game/O_RPG/OpenRPG_Stats/Structs/s_AttributesSaveData Structure"))
  (return (make `/Game/O_RPG/OpenRPG_Stats/Structs/s_AttributesSaveData` (`self.Attributes`) (`self.AvailableAttributePoints`) (`self.SpentAttributePoints`))))

(fn `GetAttributesData`
  (returns (Data :type "/Game/O_RPG/OpenRPG_Stats/Structs/s_AttributesData Structure"))
  (bind _returnvalue (`|GetDataTableRow` (`self.AttributesTable`) (`self.AttributesTableRow`))
    (:`then`
      (return _returnvalue))
    (:`RowNotFound`
      (return))))

(fn `GetAttributeValue`
  (params (Attribute :type "/Game/O_RPG/OpenRPG_Stats/Enums/e_Attribute Enum" :default "NewEnumerator6"))
  (returns (Value :type Integer))
  ;[0.02628 1 0.4395] Gets the calculated final value of the input attribute
  (return (`.FinalValue_9_4273F5764C3DF52F895994A4ED72F50D` (break `/Game/O_RPG/OpenRPG_Stats/Structs/s_Attribute` (`BlueprintMapLibrary.Map_Find` (`self.Attributes`) Attribute)))))

(fn `LoadData`
  (params (SaveName :type String) (`FromGameInstance?` :type Boolean))
  (locals (LocalSavedData :type "/Game/O_RPG/OpenRPG_Stats/Structs/s_AttributesSaveData Structure") (LocalSaveName :type String) (LocalSaveObject :type "/Game/O_RPG/OpenRPG_Stats/Blueprints/BP_StatsSaveObject Object Reference"))
  (bind (_savedattributes _savedavailableattributepoints _savedspentattributepoints) (break `/Game/O_RPG/OpenRPG_Stats/Structs/s_AttributesSaveData` (`local.LocalSavedData`)))
  (set `local.LocalSaveName` SaveName)
  (if `FromGameInstance?`
    (bind (_found_ _data) (message `/Game/O_RPG/OpenRPG_Stats/Blueprints/Interfaces/BP_SaveLoad.LoadAttributes` (`GameplayStatics.GetGameInstance`) (`local.LocalSaveName`)))
    (if _found_
      (set `local.LocalSavedData` _data)
      (else
        (return)))
    (else
      (bind _output_get (set `local.LocalSaveObject` (`/Game/O_RPG/OpenRPG_Stats/Blueprints/BPL_Stats.GetStatsSaveObject`)))
      (`/Engine/EditorBlueprintResources/StandardMacros.IsValid` _output_get
        (:`Is Valid`
          (bind (_found__2 _data_2) (message `/Game/O_RPG/OpenRPG_Stats/Blueprints/Interfaces/BP_SaveLoad.LoadAttributes` (`local.LocalSaveObject`) (`local.LocalSaveName`)))
          (if _found__2
            (set `local.LocalSavedData` _data_2)
            (else
              (return))))
        (:`Is Not Valid`
          (return)))))
  (set `self.Attributes` _savedattributes)
  (set `self.AvailableAttributePoints` _savedavailableattributepoints)
  (set `self.SpentAttributePoints` _savedspentattributepoints)
  (set `self.HasLoadBeenSuccessful?` true)
  (return))

(fn `LoadTableData`
  (locals (LocalAttributesData :type "/Game/O_RPG/OpenRPG_Stats/Structs/s_AttributesData Structure") (LocalDefaultAttributes :type "Map of /Game/O_RPG/OpenRPG_Stats/Enums/e_Attribute Enum to Integer") (LocalAttribute :type "/Game/O_RPG/OpenRPG_Stats/Enums/e_Attribute Enum") (`LocalPreviousSuccess?` :type Boolean))
  (`/Engine/EditorBlueprintResources/StandardMacros.IsValid` (`self.AttributesTable`)
    (:`Is Valid`
      (bind _output_get (set `local.LocalDefaultAttributes` (`.Attributes_16_BA76E1204E2CD013510F85AB363740DC` (break `/Game/O_RPG/OpenRPG_Stats/Structs/s_AttributesData` (`self.GetAttributesData`)))))
      (bind _keys (`BlueprintMapLibrary.Map_Keys` _output_get))
      (for _array_element _keys
        (bind _output_get_2 (set `local.LocalAttribute` _array_element))
        (bind _value (`BlueprintMapLibrary.Map_Find` (`local.LocalDefaultAttributes`) _output_get_2))
        (`BlueprintMapLibrary.Map_Add` (`self.Attributes`) (`local.LocalAttribute`) (make `/Game/O_RPG/OpenRPG_Stats/Structs/s_Attribute` :`BaseValue` _value :`FinalValue` _value)))
      (return))
    (:`Is Not Valid`
      (return))))

(fn `ReceiveAttributePoints`
  (params (Points :type Integer))
  (locals (LocalPoints :type Integer))
  (bind _output_get (set `local.LocalPoints` Points))
  (if (!= _output_get 0)
    (bind _output_get_2 (set `self.AvailableAttributePoints` (+ (`local.LocalPoints`) (`self.AvailableAttributePoints`))))
    (`self.UpdateAttributePoints` _output_get_2)
    (`self.OnAttributePointsReceived` (`local.LocalPoints`) (`self.AvailableAttributePoints`))
    (return)
    (else
      (return))))

(fn `RefreshWidgets`
  (bind _keys (`BlueprintMapLibrary.Map_Keys` (`self.Attributes`)))
  (for _array_element _keys
    (`self.UpdateAttributeValue` _array_element (`self.GetAttributeValue` _array_element)))
  (`self.UpdateAttributePoints` (`self.AvailableAttributePoints`))
  (return))

(fn `RemoveAttributeBonuses`
  (params (AttributeBonuses :type "/Game/O_RPG/OpenRPG_Stats/Structs/s_AttributeBonus Structure"))
  (locals (LocalFlatBonuses :type "Map of /Game/O_RPG/OpenRPG_Stats/Enums/e_Attribute Enum to Float (double-precision)") (LocalPercentageBonuses :type "Map of /Game/O_RPG/OpenRPG_Stats/Enums/e_Attribute Enum to Float (double-precision)") (LocalCurrentLoopAttribute :type "/Game/O_RPG/OpenRPG_Stats/Enums/e_Attribute Enum") (LocalCurrentLoopAttributeData :type "/Game/O_RPG/OpenRPG_Stats/Structs/s_Attribute Structure") (LocalModifiedAttributes :type "Array of /Game/O_RPG/OpenRPG_Stats/Enums/e_Attribute Enum"))
  (bind (_flatbonuses _percentagebonuses) (break `/Game/O_RPG/OpenRPG_Stats/Structs/s_AttributeBonus` AttributeBonuses))
  (set `local.LocalFlatBonuses` _flatbonuses)
  (set `local.LocalPercentageBonuses` _percentagebonuses)
  (bind _keys (`BlueprintMapLibrary.Map_Keys` (`local.LocalFlatBonuses`)))
  (bind _output_get (set `local.LocalModifiedAttributes` _keys))
  (for _array_element _output_get
    (bind _output_get_2 (set `local.LocalCurrentLoopAttribute` _array_element))
    (bind _output_get_3 (set `local.LocalCurrentLoopAttributeData` (`BlueprintMapLibrary.Map_Find` (`self.Attributes`) _output_get_2)))
    (bind _structout (setmembers `/Game/O_RPG/OpenRPG_Stats/Structs/s_Attribute` :`StructRef` _output_get_3 :`FlatBonuses` (- (`.FlatBonuses_28_3F6008684D9845B3258C57AB96242FE5` (break `/Game/O_RPG/OpenRPG_Stats/Structs/s_Attribute` _output_get_3)) (`BlueprintMapLibrary.Map_Find` (`local.LocalFlatBonuses`) (`local.LocalCurrentLoopAttribute`)))))
    (`BlueprintMapLibrary.Map_Add` (`self.Attributes`) (`local.LocalCurrentLoopAttribute`) _structout))
  (bind _keys_2 (`BlueprintMapLibrary.Map_Keys` (`local.LocalPercentageBonuses`)))
  (for _array_element_2 _keys_2
    (bind _output_get_4 (set `local.LocalCurrentLoopAttribute` _array_element_2))
    (bind _output_get_5 (set `local.LocalCurrentLoopAttributeData` (`BlueprintMapLibrary.Map_Find` (`self.Attributes`) _output_get_4)))
    (bind _structout_2 (setmembers `/Game/O_RPG/OpenRPG_Stats/Structs/s_Attribute` :`StructRef` _output_get_5 :`PercentageBonuses` (- (`.PercentageBonuses_29_4A36E47747DB8544BA56E4AF979B4155` (break `/Game/O_RPG/OpenRPG_Stats/Structs/s_Attribute` _output_get_5)) (`BlueprintMapLibrary.Map_Find` (`local.LocalPercentageBonuses`) (`local.LocalCurrentLoopAttribute`)))))
    (`BlueprintMapLibrary.Map_Add` (`self.Attributes`) (`local.LocalCurrentLoopAttribute`) _structout_2)
    (`KismetArrayLibrary.Array_AddUnique` (`local.LocalModifiedAttributes`) (`local.LocalCurrentLoopAttribute`)))
  (`self.CalculateAttributesFinalValues` (`local.LocalModifiedAttributes`))
  (return))

(fn `ResetAttributes`
  (locals (LocalAttributesData :type "/Game/O_RPG/OpenRPG_Stats/Structs/s_AttributesData Structure") (LocalDefaultAttributes :type "Map of /Game/O_RPG/OpenRPG_Stats/Enums/e_Attribute Enum to Integer") (LocalCurrentLoopAttribute :type "/Game/O_RPG/OpenRPG_Stats/Enums/e_Attribute Enum"))
  (`/Engine/EditorBlueprintResources/StandardMacros.IsValid` (`self.AttributesTable`)
    (:`Is Valid`
      (bind _output_get (set `local.LocalAttributesData` (`self.GetAttributesData`)))
      (bind _output_get_2 (set `local.LocalDefaultAttributes` (`.Attributes_16_BA76E1204E2CD013510F85AB363740DC` (break `/Game/O_RPG/OpenRPG_Stats/Structs/s_AttributesData` _output_get))))
      (bind _keys (`BlueprintMapLibrary.Map_Keys` _output_get_2))
      (for _array_element _keys
        (bind _output_get_3 (set `local.LocalCurrentLoopAttribute` _array_element))
        (`self.AddPointsToAttribute` (`local.LocalCurrentLoopAttribute`) (- (`BlueprintMapLibrary.Map_Find` (`local.LocalDefaultAttributes`) _output_get_3) (`.BaseValue_5_5398D8464682C14444DF888899E8366F` (break `/Game/O_RPG/OpenRPG_Stats/Structs/s_Attribute` (`BlueprintMapLibrary.Map_Find` (`self.Attributes`) (`local.LocalCurrentLoopAttribute`)))))) ; Points will be negative
      )
      (`self.ReceiveAttributePoints` (`self.SpentAttributePoints`))
      (set `self.SpentAttributePoints` 0)
      (`self.OnAttributesResetted`)
      (return))
    (:`Is Not Valid`
      (return))))

(fn `SaveData`
  (params (SaveName :type String) (`ToGameInstance?` :type Boolean))
  (returns (`Success?` :type Boolean))
  (locals (LocalSaveName :type String) (LocalSaveObject :type "/Game/O_RPG/OpenRPG_Stats/Blueprints/BP_StatsSaveObject Object Reference"))
  (set `local.LocalSaveName` SaveName)
  (if `ToGameInstance?`
    (message `/Game/O_RPG/OpenRPG_Stats/Blueprints/Interfaces/BP_SaveLoad.SaveAttributes` (`GameplayStatics.GetGameInstance`) (`local.LocalSaveName`) (`self.CreateSaveData`))
    (return true)
    (else
      (bind _output_get (set `local.LocalSaveObject` (`/Game/O_RPG/OpenRPG_Stats/Blueprints/BPL_Stats.GetStatsSaveObject`)))
      (`/Engine/EditorBlueprintResources/StandardMacros.IsValid` _output_get
        (:`Is Valid`
          (message `/Game/O_RPG/OpenRPG_Stats/Blueprints/Interfaces/BP_SaveLoad.SaveAttributes` (`local.LocalSaveObject`) (`local.LocalSaveName`) (`self.CreateSaveData`))
          (bind _returnvalue (`GameplayStatics.SaveGameToSlot` (`local.LocalSaveObject`) (`/Game/O_RPG/OpenRPG_Stats/Blueprints/BPL_Stats.GetStatsSlotName`)))
          (return _returnvalue))
        (:`Is Not Valid`
          (return false))))))

(fn `SpendAttributePoints`
  (params (Attribute :type "/Game/O_RPG/OpenRPG_Stats/Enums/e_Attribute Enum" :default "NewEnumerator6") (Points :type Integer))
  (locals (LocalAttribute :type "/Game/O_RPG/OpenRPG_Stats/Enums/e_Attribute Enum") (LocalPoints :type Integer))
  (bind _localattribute (`local.LocalAttribute`))
  ;[0.8861 1 0.09855] Called when the "+" button is pressed in the UI when there are available attribute points to spend. It calls AddPointsToAttribute which handles all the calculations and then adjusts the AvailableAttributePoints and SpentAttributePoints variables.
  (set `local.LocalAttribute` Attribute)
  (bind _output_get (set `local.LocalPoints` Points))
  (if (!= _output_get 0)
    (`self.AddPointsToAttribute` (`local.LocalAttribute`) (`local.LocalPoints`))
    (set `self.AvailableAttributePoints` (- (`self.AvailableAttributePoints`) (`local.LocalPoints`)))
    (set `self.SpentAttributePoints` (+ (`self.SpentAttributePoints`) (`local.LocalPoints`)))
    (`self.UpdateAttributePoints` (`self.AvailableAttributePoints`))
    (`self.UpdateAttributeValue` _localattribute (`self.GetAttributeValue` _localattribute))
    (`self.OnAttributePointsSpent` (`local.LocalAttribute`) (`local.LocalPoints`) (`self.AvailableAttributePoints`))
    (return)
    (else
      (return))))