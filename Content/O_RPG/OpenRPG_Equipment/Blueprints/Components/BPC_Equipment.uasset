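; Equipment component that tracks one item per slot type on the player and moves items between slots and inventory containers, including swaps and drops.
; Equipping and unequipping update the owner's per-slot skeletal meshes via leader pose or socket attachment, then the slot map, UI and dispatchers.
; Initialization validates the owner's interface setup and polls until the UI widget exists.
; Saving and loading go through a GameInstance interface; loading respawns item actors and re-equips.
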(event `Initialize`
  ;[0.03839 0.3633 1] The initialization process basically consists in checking that everything seems to be configured successfully, then it gets the equipment widget and updates it with the equipped items (for example if we have loaded something previously)
  (bind _success_ (`self.CheckConsistency`))
  (if _success_
    ;;[0.06569 0.07899 1] Just in case the player controller hast finished creating the widgets
    (bind _widget (message `/Game/O_RPG/OpenRPG_Equipment/Blueprints/Interfaces/BPI_EquipmentWidgets.GetMainEquipmentWidget` (`GameplayStatics.GetPlayerController` 0) :!label _label))
    (bind _output_get (set `self.MainEquipmentWidget` _widget))
    (`/Engine/EditorBlueprintResources/StandardMacros.IsValid` _output_get
      (:`Is Valid`
        (bind _widget_2 (message `/Game/O_RPG/OpenRPG_Equipment/Blueprints/Interfaces/BPI_EquipmentWidgets.GetEquipmentContainerWidget` (`GameplayStatics.GetPlayerController` 0)))
        (bind _output_get_2 (set `self.EquipmentSlotsContainerWidget` _widget_2))
        (`/Engine/EditorBlueprintResources/StandardMacros.IsValid` _output_get_2
          (:`Is Valid`
            (`/Game/O_RPG/OpenRPG_Equipment/Widgets/WB_EquipmentSlotsContainer.Initialize` (`self.EquipmentSlotsContainerWidget`) self)
            (`self.PrintDebug` "Equipment: Initialized successfully!" (struct :`R` 0.082484 :`G` 1.0 :`A` 1.0) 3.0))
          (:`Is Not Valid`
            (`self.PrintDebug` "Equipment: GetEquipmentContainer isnt returning a valid container widget during initialization" (struct :`R` 1.0 :`A` 1.0) 6.0))))
      (:`Is Not Valid`
        (`self.PrintDebug` "Trying to get main equipment container widget..." (struct :`G` 0.395769 :`B` 1.0 :`A` 1.0) 0.2)
        (`KismetSystemLibrary.Delay` 0.05)
        (goto _label)))))

(event `UpdateEquipmentSlot`
  (params (Slot :type "/Game/O_RPG/OpenRPG_Equipment/Enums/e_EquipmentType Enum" :default "NewEnumerator0"))
  (bind _equipmentslotscontainerwidget (`self.EquipmentSlotsContainerWidget`))
  ;[1 0.4218 0.1063] Called when we want to update one slot from the UI
  (`/Engine/EditorBlueprintResources/StandardMacros.IsValid` _equipmentslotscontainerwidget
    (:`Is Valid`
      (`/Game/O_RPG/OpenRPG_Equipment/Widgets/WB_EquipmentSlotsContainer.UpdateSlot` _equipmentslotscontainerwidget Slot))))

(fn `CheckConsistency`
  (returns (`Success?` :type Boolean))
  (if (`KismetSystemLibrary.DoesImplementInterface` (`self.GetOwner`) "/Game/O_RPG/OpenRPG_Equipment/Blueprints/Interfaces/BPI_Equipment.BPI_Equipment_C")
    (`/Engine/EditorBlueprintResources/StandardMacros.IsValid` (`/Game/O_RPG/OpenRPG_Inventory/Blueprints/Library/BPL_Inventory.GetPlayerInventory`)
      (:`Is Valid`
        (bind _mesh (message `/Game/O_RPG/OpenRPG_Equipment/Blueprints/Interfaces/BPI_Equipment.GetMesh` (`self.GetOwner`)))
        (`/Engine/EditorBlueprintResources/StandardMacros.IsValid` _mesh
          (:`Is Valid`
            (bind _enumvalue (foreach `/Game/O_RPG/OpenRPG_Equipment/Enums/e_EquipmentType` false)
              (:`LoopBody`
                (if (`|EnumInequality` _enumvalue "NewEnumerator8")
                  (bind _meshcomponent (message `/Game/O_RPG/OpenRPG_Equipment/Blueprints/Interfaces/BPI_Equipment.GetEquipmentMeshComponentByType` (`self.GetOwner`) _enumvalue))
                  (`/Engine/EditorBlueprintResources/StandardMacros.IsValid` _meshcomponent
                    (:`Is Not Valid`
                      (`self.PrintDebug` (`KismetStringLibrary.Concat_StrStr` "Equipment: Item equipping aborted, the interface function GetEquipmentMeshComponentByType isnt returning a valid mesh component. for the slot " (`|GetEnumeratorNameAsString` _enumvalue)) (struct :`R` 0.869792 :`G` 0.031711 :`B` 0.031711 :`A` 1.0) 10.0)
                      (return false)))))
              (:`then`
                (return true))))
          (:`Is Not Valid`
            (`self.PrintDebug` "Equipment: Item equipping aborted, the interface function GetPlayerMesh isnt returning a valid mesh component. Make sure you have implemented it!" (struct :`R` 0.869792 :`G` 0.031711 :`B` 0.031711 :`A` 1.0) 10.0)
            (return false))))
      (:`Is Not Valid`
        (`self.PrintDebug` "Equipment Your player doesnt have the PlayerInventory component" (struct :`R` 0.994792 :`G` 0.070239 :`A` 1.0) 5.0)
        (return false)))
    (else
      (`self.PrintDebug` "Equipment Your player doesnt implement the BPL_Equipment interface" (struct :`R` 0.994792 :`G` 0.070239 :`A` 1.0) 5.0)
      (return false))))

(fn `CreateEquipmentSaveData`
  (returns (Data :type "/Game/O_RPG/OpenRPG_Equipment/Structs/s_EquipmentSaveData Structure"))
  (return (make `/Game/O_RPG/OpenRPG_Equipment/Structs/s_EquipmentSaveData` (`self.Equipment`))))

(fn `EquipFromContainer`
  (params (FromContainer :type "/Game/O_RPG/OpenRPG_Inventory/Blueprints/Components/BPC_ItemsContainer Object Reference") (FromIndex :type Integer))
  (returns (`Success?` :type Boolean))
  (locals (LocalFromContainer :type "/Game/O_RPG/OpenRPG_Inventory/Blueprints/Components/BPC_ItemsContainer Object Reference") (LocalFromIndex :type Integer) (LocalItemToEquip :type Name) (LocalEquippedItem :type Name) (LocalSlotType :type "/Game/O_RPG/OpenRPG_Equipment/Enums/e_EquipmentType Enum" :default "NewEnumerator0") (LocalUnequipped :type Boolean))
  (set `local.LocalFromContainer` FromContainer)
  (set `local.LocalFromIndex` FromIndex)
  ;[0.1949 0.01829 1] Perform all the necessary checks
  (`/Engine/EditorBlueprintResources/StandardMacros.IsValid` (`local.LocalFromContainer`)
    (:`Is Valid`
      (bind _output_get (set `local.LocalItemToEquip` (`.Item_8_78E0EFF340AA0567F5C6C3BC6148D1F0` (break `/Game/O_RPG/OpenRPG_Inventory/Structs/s_InventoryItem` (`/Game/O_RPG/OpenRPG_Inventory/Blueprints/Components/BPC_ItemsContainer.GetItemAtIndex` (`local.LocalFromContainer`) (`local.LocalFromIndex`))))))
      (if (!= _output_get "None")
        (bind _output_get_2 (set `local.LocalSlotType` (`.Type_2_DA36326348B1744870DE2FABC5024214` (break `/Game/O_RPG/OpenRPG_Equipment/Structs/s_EquipmentData` (`self.GetEquipmentDataFromItem` (`local.LocalItemToEquip`))))))
        (if (`|EnumInequality` _output_get_2 "NewEnumerator8")
          ;[0.1521 0.3289 1] Check if we have something already equipped in the slot we want to equip
          (bind _output_get_3 (set `local.LocalEquippedItem` (`self.GetSlotItem` (`local.LocalSlotType`)))) ; Get the equipped item in that particular slot
          (if (not (== _output_get_3 "None"))
            ;[0.1197 0.6949 1] There is an item already equipped, so we need to unequip it to the slot index of the item we want to equip, but first its necessary to clear the slot of that item, so the unequip can be done without problems. With the item unequipped, we can now equip the item we holded in the LocalItemToEquip variable
            (`/Game/O_RPG/OpenRPG_Inventory/Blueprints/Components/BPC_ItemsContainer.RemoveIndexAmount` (`local.LocalFromContainer`) (`local.LocalFromIndex`) 1)
            (bind _success_ (`self.UnequipItem` (`local.LocalSlotType`) (`local.LocalFromContainer`) (`local.LocalFromIndex`)))
            (set `local.LocalUnequipped` _success_))
          ;[0.7991 0.3176 1] Then equip the item, its not going to fail because we know the item has a valid equipment slot
          (`self.EquipItem` (`local.LocalItemToEquip`))
          ;[0.8861 1 0.09855] Finally we just need an extra check because if we didnt have to unequip the item, then we need to remove the item from the inventory as its supposed to be "transfered" from the inventory to the equipment
          (if (not (`local.LocalUnequipped`))
            (`/Game/O_RPG/OpenRPG_Inventory/Blueprints/Components/BPC_ItemsContainer.RemoveIndexAmount` (`local.LocalFromContainer`) (`local.LocalFromIndex`) 1))
          (return true)
          (else
            (`self.PrintDebug` "Equipment: Trying to equip an item with no valid equipment slot assigned" (struct :`R` 1.0 :`A` 1.0) 6.0)
            (return false)))
        (else
          (`self.PrintDebug` "Equipment: FromIndex parameters seems to be not valid one" (struct :`R` 1.0 :`A` 1.0) 6.0)
          (return false))))
    (:`Is Not Valid`
      (`self.PrintDebug` "Equipment: FromContainer parameter not valid in function EquipFromContainer" (struct :`R` 1.0 :`A` 1.0) 6.0)
      (return false))))

(fn `EquipItem`
  (params (Item :type Name))
  (returns (`Success?` :type Boolean))
  (locals (LocalEquipmentData :type "/Game/O_RPG/OpenRPG_Equipment/Structs/s_EquipmentData Structure") (LocalSlotType :type "/Game/O_RPG/OpenRPG_Equipment/Enums/e_EquipmentType Enum") (LocalItem :type Name))
  ;[0.2843 0.1367 1] Get the info for that item
  (bind _output_get (set `local.LocalItem` Item))
  (bind _output_get_2 (set `local.LocalEquipmentData` (`self.GetEquipmentDataFromItem` _output_get)))
  ;[0.1622 1 0.28] Make sure the slot is valid
  (bind _output_get_3 (set `local.LocalSlotType` (`.Type_2_DA36326348B1744870DE2FABC5024214` (break `/Game/O_RPG/OpenRPG_Equipment/Structs/s_EquipmentData` _output_get_2))))
  (if (`|EnumInequality` _output_get_3 "NewEnumerator8")
    ;[0.09621 0.6087 1] Update the visuals with that new item
    (`self.UpdateEquipmentVisuals` (`local.LocalEquipmentData`) true)
    ;[1 0.05203 0.06197] Finally update data structures and UI, and throw a dispatcher
    (`BlueprintMapLibrary.Map_Add` (`self.Equipment`) (`local.LocalSlotType`) (`local.LocalItem`))
    (`self.UpdateEquipmentSlot` (`local.LocalSlotType`))
    (`self.OnItemEquipped` (`local.LocalItem`) (`local.LocalSlotType`))
    (return true)
    (else
      (`self.PrintDebug` "Equipment: Cant equip a non equipment item" (struct :`R` 0.869792 :`G` 0.031711 :`B` 0.031711 :`A` 1.0) 5.0)
      (return false))))

(fn `EquipLoadedEquipment`
  (params (Data :type "/Game/O_RPG/OpenRPG_Equipment/Structs/s_EquipmentSaveData Structure"))
  (locals (LocalSavedEquipment :type "Map of /Game/O_RPG/OpenRPG_Equipment/Enums/e_EquipmentType Enum to Name") (LocalItem :type Name) (LocalItemData :type "/Game/O_RPG/OpenRPG_Inventory/Structs/s_ItemData Structure") (LocalPlayerInventory :type "/Game/O_RPG/OpenRPG_Inventory/Blueprints/Components/BPC_PlayerInventory Object Reference"))
  (set `local.LocalSavedEquipment` (`.SavedEquipment_5_F551ADF9485569B3B83A1CB2C5544957` (break `/Game/O_RPG/OpenRPG_Equipment/Structs/s_EquipmentSaveData` Data)))
  (set `local.LocalPlayerInventory` (`/Game/O_RPG/OpenRPG_Inventory/Blueprints/Library/BPL_Inventory.GetPlayerInventory`))
  (bind _keys (`BlueprintMapLibrary.Map_Keys` (`local.LocalSavedEquipment`)))
  (for _array_element _keys
    (bind _output_get (set `local.LocalItem` (`BlueprintMapLibrary.Map_Find` (`local.LocalSavedEquipment`) _array_element)))
    (bind _output_get_2 (set `local.LocalItemData` (`/Game/O_RPG/OpenRPG_Inventory/Blueprints/Library/BPL_Inventory.GetItemDataByRow` _output_get)))
    (bind ((`Class_47_1920DEDC49E9F940C8E7B5830EF818FF` _class)) (break `/Game/O_RPG/OpenRPG_Inventory/Structs/s_ItemData` _output_get_2))
    (if (`KismetSystemLibrary.IsValidClass` _class)
      (bind _returnvalue (`|SpawnActorFromClass` _class (`KismetMathLibrary.MakeTransform` (0.0 0.0 0.0)) "Undefined" "SelectDefaultAtRuntime" null (`local.LocalItem`) null (`local.LocalItemData`)))
      (`/Game/O_RPG/OpenRPG_Inventory/Blueprints/Components/BPC_PlayerInventory.AddSpawnedActor` (`local.LocalPlayerInventory`) (`local.LocalItem`) _returnvalue))
    (`self.EquipItem` (`local.LocalItem`)))
  (return))

(fn `GetEquipmentDataFromItem`
  (params (Item :type Name))
  (returns (EquipmentData :type "/Game/O_RPG/OpenRPG_Equipment/Structs/s_EquipmentData Structure"))
  (locals (LocalItem :type Name))
  (return (`/Game/O_RPG/OpenRPG_Equipment/Blueprints/Library/BPL_Equipment.GetEquipmentDataByRow` (`.EquipmentDataRowName_65_6F8B33B44342009084580493709A417C` (break `/Game/O_RPG/OpenRPG_Inventory/Structs/s_ItemData` (`/Game/O_RPG/OpenRPG_Inventory/Blueprints/Library/BPL_Inventory.GetItemDataByRow` Item))))))

(fn `GetSlotItem`
  (params (SlotType :type "/Game/O_RPG/OpenRPG_Equipment/Enums/e_EquipmentType Enum" :default "NewEnumerator0"))
  (returns (Item :type Name))
  (locals (LocalSlot :type "/Game/O_RPG/OpenRPG_Equipment/Enums/e_EquipmentType Enum") (LocalItemID :type Integer))
  (return (`BlueprintMapLibrary.Map_Find` (`self.Equipment`) SlotType)))

(fn `LoadEquipment`
  (params (SaveName :type String))
  (returns (`Success?` :type Boolean))
  (locals (LocalSaveName :type String) (`LocalFromGameInstance?` :type Boolean) (LocalSaveContainer :type "Object Object Reference") (LocalUserIndex :type Integer))
  (bind _localsavename (`local.LocalSaveName`))
  (set `local.LocalSaveName` SaveName)
  (if (`KismetSystemLibrary.DoesImplementInterface` (`GameplayStatics.GetGameInstance`) "/Game/O_RPG/OpenRPG_Equipment/Blueprints/Interfaces/BPI_EquipmentSave.BPI_EquipmentSave_C")
    (bind (_found_ _data) (message `/Game/O_RPG/OpenRPG_Equipment/Blueprints/Interfaces/BPI_EquipmentSave.LoadEquipment` (`GameplayStatics.GetGameInstance`) _localsavename))
    (if _found_
      (`self.EquipLoadedEquipment` _data)
      (return true)
      (else
        (`self.PrintDebug` (`KismetStringLibrary.Concat_StrStr` "Loading equipment aborted, LoadEquipment function hasnt found any save data in save container with save name " _localsavename) (struct :`R` 0.96875 :`G` 0.035319 :`B` 0.035319 :`A` 1.0) 6.0)
        (return false)))
    (else
      (`self.PrintDebug` (`KismetStringLibrary.Concat_StrStr` "Error while saving equipment, GameInstance" "doesnt implement the interface BPI_EquipmentSave") (struct :`R` 0.96875 :`G` 0.035319 :`B` 0.035319 :`A` 1.0) 6.0)
      (return false))))

(fn `SaveEquipment`
  (params (SaveName :type String))
  (returns (`Success?` :type Boolean))
  (locals (LocalSaveName :type String))
  (set `local.LocalSaveName` SaveName)
  (if (`KismetSystemLibrary.DoesImplementInterface` (`GameplayStatics.GetGameInstance`) "/Game/O_RPG/OpenRPG_Equipment/Blueprints/Interfaces/BPI_EquipmentSave.BPI_EquipmentSave_C")
    (message `/Game/O_RPG/OpenRPG_Equipment/Blueprints/Interfaces/BPI_EquipmentSave.SaveEquipment` (`GameplayStatics.GetGameInstance`) (`local.LocalSaveName`) (`self.CreateEquipmentSaveData`))
    (return true)
    (else
      (`self.PrintDebug` (`KismetStringLibrary.Concat_StrStr` "Error while saving equipment, GameInstance " "doesnt implement the interface BPI_EquipmentSave") (struct :`R` 0.96875 :`G` 0.035319 :`B` 0.035319 :`A` 1.0) 6.0)
      (return false))))

(fn `UnequipItem`
  (params (SlotType :type "/Game/O_RPG/OpenRPG_Equipment/Enums/e_EquipmentType Enum" :default "NewEnumerator0") (ToContainer :type "/Game/O_RPG/OpenRPG_Inventory/Blueprints/Components/BPC_ItemsContainer Object Reference") (ToSpecificInventoryIndex :type Integer) (`Drop?` :type Boolean))
  (returns (`Success?` :type Boolean))
  (locals (LocalSlotType :type "/Game/O_RPG/OpenRPG_Equipment/Enums/e_EquipmentType Enum") (LocalSpecificIndex :type Integer) (LocalDrop :type Boolean) (LocalMeshComponent :type "SkeletalMeshComponent Object Reference") (LocalEquippedItem :type Name :default "None") (LocalToContainer :type "/Game/O_RPG/OpenRPG_Inventory/Blueprints/Components/BPC_ItemsContainer Object Reference"))
  (set `local.LocalSlotType` SlotType)
  (set `local.LocalToContainer` ToContainer)
  (set `local.LocalSpecificIndex` ToSpecificInventoryIndex)
  (set `local.LocalDrop` `Drop?`)
  ;[0.2642 1 0.1392] Check the slot is valid
  (if (`|EnumInequality` (`local.LocalSlotType`) "NewEnumerator8")
    (set `local.LocalEquippedItem` (`self.GetSlotItem` (`local.LocalSlotType`)))
    (if (`local.LocalDrop`)
      (`/Game/O_RPG/OpenRPG_Inventory/Blueprints/Components/BPC_ItemsContainer.DropItem` (`local.LocalToContainer`) (make `/Game/O_RPG/OpenRPG_Inventory/Structs/s_InventoryItem` (`local.LocalEquippedItem`) 1)) ; Then drop it
      (else
        ;[0.07462 1 0.09289] First lets check if the destination container is a valid one
        (`/Engine/EditorBlueprintResources/StandardMacros.IsValid` (`local.LocalToContainer`)
          (:`Is Valid`
            (if (== (`local.LocalSpecificIndex`) -1)
              ;[0.07902 0.3304 1] Unequipping to any empty slot of the destination container, so if we can just add it we are done, otherwise abort the operation
              (bind _success_ (`/Game/O_RPG/OpenRPG_Inventory/Blueprints/Components/BPC_ItemsContainer.AddItem` (`local.LocalToContainer`) (make `/Game/O_RPG/OpenRPG_Inventory/Structs/s_InventoryItem` (`local.LocalEquippedItem`) 1)))
              (if _success_
                _
                (else
                  (`self.PrintDebug` "Equipment: Item unequipping aborted, AddItem function failed, maybe not enough space in inventory" (struct :`R` 0.869792 :`G` 0.031711 :`B` 0.031711 :`A` 1.0) 6.0)
                  (return false)))
              (else
                (bind _success__2 (`/Game/O_RPG/OpenRPG_Inventory/Blueprints/Components/BPC_ItemsContainer.AddItemToIndex` (`local.LocalToContainer`) (make `/Game/O_RPG/OpenRPG_Inventory/Structs/s_InventoryItem` (`local.LocalEquippedItem`) 1) (`local.LocalSpecificIndex`))) ; Lets try to add to that particular slot
                (if _success__2
                  _
                  (else
                    ;[1 0.6274 0.07485] If it wasnt possible to add to that specific slot its because there is another item, so lets check if the equipment slot for that particular item in that slot is the same as the one we want to unequip (so its a valid one) and if so we can perform a swap that will be made by the EquipFromContainer function
                    (if (== (`.Type_2_DA36326348B1744870DE2FABC5024214` (break `/Game/O_RPG/OpenRPG_Equipment/Structs/s_EquipmentData` (`self.GetEquipmentDataFromItem` (`.Item_8_78E0EFF340AA0567F5C6C3BC6148D1F0` (break `/Game/O_RPG/OpenRPG_Inventory/Structs/s_InventoryItem` (`/Game/O_RPG/OpenRPG_Inventory/Blueprints/Components/BPC_ItemsContainer.GetItemAtIndex` (`local.LocalToContainer`) (`local.LocalSpecificIndex`))))))) (`local.LocalSlotType`))
                      (bind _success__3 (`self.EquipFromContainer` (`local.LocalToContainer`) (`local.LocalSpecificIndex`)))
                      (return _success__3)
                      (else
                        (return false))))))))
          (:`Is Not Valid`
            (`self.PrintDebug` "Equipment: Item unequipping aborted, the destination container is not valid!" (struct :`R` 0.869792 :`G` 0.031711 :`B` 0.031711 :`A` 1.0) 6.0)
            (return false)))))
    ;[0.155 0.5724 1] Clear the visuals
    (`self.UpdateEquipmentVisuals` (`self.GetEquipmentDataFromItem` (`local.LocalEquippedItem`)))
    ;[1 0.05203 0.06197] Finally update data structures and UI, and throw a dispatcher
    (`BlueprintMapLibrary.Map_Remove` (`self.Equipment`) (`local.LocalSlotType`))
    (`self.UpdateEquipmentSlot` (`local.LocalSlotType`))
    (`self.OnItemUnequipped` (`local.LocalEquippedItem`) (`local.LocalSlotType`) (`local.LocalDrop`))
    (return true)
    (else
      (`self.PrintDebug` "Equipment: Trying to unequip an item with no valid equipment slot assigned" (struct :`R` 1.0 :`A` 1.0) 6.0)
      (return false))))

(fn `UpdateEquipmentVisuals`
  (params (EquipmentData :type "/Game/O_RPG/OpenRPG_Equipment/Structs/s_EquipmentData Structure") (`Equip?` :type Boolean))
  (locals (LocalEquipmentData :type "/Game/O_RPG/OpenRPG_Equipment/Structs/s_EquipmentData Structure") (LocalEquip :type Boolean) (LocalMeshComponent :type "SkeletalMeshComponent Object Reference") (LocalPlayerMesh :type "SkeletalMeshComponent Object Reference"))
  (set `local.LocalEquipmentData` EquipmentData)
  (set `local.LocalEquip` `Equip?`)
  (bind _meshcomponent (message `/Game/O_RPG/OpenRPG_Equipment/Blueprints/Interfaces/BPI_Equipment.GetEquipmentMeshComponentByType` (`self.GetOwner`) (`.Type_2_DA36326348B1744870DE2FABC5024214` (break `/Game/O_RPG/OpenRPG_Equipment/Structs/s_EquipmentData` (`local.LocalEquipmentData`)))))
  (set `local.LocalMeshComponent` _meshcomponent)
  (if (`local.LocalEquip`)
    (`/Engine/EditorBlueprintResources/StandardMacros.IsValid` (`.SkeletalMesh_5_5C2626654DD7C1841B971DAA1610528C` (break `/Game/O_RPG/OpenRPG_Equipment/Structs/s_EquipmentData` (`local.LocalEquipmentData`))) ; If the mesh isnt valid we skip the visual logic part
      (:`Is Valid`
        (bind _mesh (message `/Game/O_RPG/OpenRPG_Equipment/Blueprints/Interfaces/BPI_Equipment.GetMesh` (`self.GetOwner`)))
        (set `local.LocalPlayerMesh` _mesh)
        (`SkinnedMeshComponent.SetSkinnedAssetAndUpdate` (`local.LocalMeshComponent`) (`.SkeletalMesh_5_5C2626654DD7C1841B971DAA1610528C` (break `/Game/O_RPG/OpenRPG_Equipment/Structs/s_EquipmentData` (`local.LocalEquipmentData`))) true) ; We set the mesh of that component to the one in the equipment data
        (if (== (`.CustomBoneName_8_3273E45740A6D2BC082067A2F8CE6FDD` (break `/Game/O_RPG/OpenRPG_Equipment/Structs/s_EquipmentData` (`local.LocalEquipmentData`))) "None")
          (`SkinnedMeshComponent.SetLeaderPoseComponent` (`local.LocalMeshComponent`) (`local.LocalPlayerMesh`) false false) ; If the skeletal mesh has the same skeleton as our player, this function will make it to fit it
          (return)
          (else
            (`SceneComponent.K2_AttachToComponent` (`local.LocalMeshComponent`) (`local.LocalPlayerMesh`) (`.CustomBoneName_8_3273E45740A6D2BC082067A2F8CE6FDD` (break `/Game/O_RPG/OpenRPG_Equipment/Structs/s_EquipmentData` (`local.LocalEquipmentData`))) "KeepRelative" "KeepRelative" "KeepRelative" true)
            (`SceneComponent.K2_SetRelativeTransform` (`local.LocalMeshComponent`) (`.RelativeTransform_11_437208274FCF942CD94AA1BC62DBBA44` (break `/Game/O_RPG/OpenRPG_Equipment/Structs/s_EquipmentData` (`local.LocalEquipmentData`))) false false)
            (return))))
      (:`Is Not Valid`
        (return)))
    (else
      (`SkinnedMeshComponent.SetSkinnedAssetAndUpdate` (`local.LocalMeshComponent`) null true) ; Resets the visual equipment, it simulates that we unequipped the item
      (return))))