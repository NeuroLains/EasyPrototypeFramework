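; BPC_Storage is an inventory container component for storage, defining how items move between it and the player inventory.
; Clicking a slot transfers that item to the player inventory without specifying a target slot.
; Slot drops branch on the source container type: player inventory items transfer into the dropped slot, Storage sources use the self-drop handler, and Shop drops are ignored.
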(event `self.OnSlotClicked`
  (params (ClickedIndex :type Integer))
  ;[1 0.03646 0.1158] Override On Slot Clicked: In this case it just transfers the clicked index to the player inventory...
  (`self.TransferItem` (`/Game/O_RPG/OpenRPG_Inventory/Blueprints/Library/BPL_Inventory.GetPlayerInventory`) -1 ClickedIndex))

(fn `HandleSlotDrop`
  (params (FromContainer :type "/Game/O_RPG/OpenRPG_Inventory/Blueprints/Components/BPC_ItemsContainer Object Reference") (FromIndex :type Integer) (DroppedIndex :type Integer))
  (locals (LocalFromContainer :type "/Game/O_RPG/OpenRPG_Inventory/Blueprints/Components/BPC_ItemsContainer Object Reference") (LocalFromIndex :type Integer) (LocalDroppedIndex :type Integer))
  (set `local.LocalFromContainer` FromContainer)
  (set `local.LocalFromIndex` FromIndex)
  (set `local.LocalDroppedIndex` DroppedIndex)
  (switch `/Game/O_RPG/OpenRPG_Inventory/Enums/e_ContainerType` (`/Game/O_RPG/OpenRPG_Inventory/Blueprints/Components/BPC_ItemsContainer.ContainerType` (`local.LocalFromContainer`))
    (:`NewEnumerator0`
      (`self.TransferItem` (`local.LocalFromContainer`) self (`local.LocalDroppedIndex`) (`local.LocalFromIndex`))
      (return))
    (:`NewEnumerator1`
      (`self.HandleSelfSlotDrop` (`local.LocalFromIndex`) (`local.LocalDroppedIndex`))
      (return))
    (:`NewEnumerator2`
      (return))))