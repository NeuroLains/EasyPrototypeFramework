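; BPL_Inventory is a Blueprint function library of shared helpers for the RPG inventory system.
; It fetches the BPC_PlayerInventory component from player character 0 and maps item rarity to a fixed color.
; Row-name lookups return item data from DT_Items or item lists from DT_ItemsList, with empty results when a row is missing.
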(fn `GetColorByItemRarity`
  (params (Rarity :type "/Game/O_RPG/OpenRPG_Inventory/Enums/e_ItemRarity Enum" :default "NewEnumerator0"))
  (returns (Color :type "LinearColor Structure"))
  (return (select `/Game/O_RPG/OpenRPG_Inventory/Enums/e_ItemRarity` Rarity :`NewEnumerator0` (struct :`R` 0.033112 :`G` 0.401042 :`B` 0.324646 :`A` 1.0) :`NewEnumerator1` (struct :`R` 0.210604 :`G` 0.671875 :`B` 0.103083 :`A` 1.0) :`NewEnumerator2` (struct :`R` 1.0 :`G` 0.028639 :`A` 1.0) :`NewEnumerator3` (struct :`R` 0.442708 :`G` 0.263895 :`B` 0.015424 :`A` 1.0) :`NewEnumerator4` (struct :`G` 0.232847 :`B` 1.0 :`A` 1.0) :!type "LinearColor Structure")))

(fn `GetItemDataByRow`
  (params (Item :type Name))
  (returns (Data :type "/Game/O_RPG/OpenRPG_Inventory/Structs/s_ItemData Structure"))
  (bind _returnvalue (`|GetDataTableRow` "/Game/O_RPG/OpenRPG_Inventory/Datatables/DT_Items.DT_Items" Item)
    (:`then`
      (return _returnvalue))
    (:`RowNotFound`
      (return))))

(fn `GetItemsListByRow`
  (params (Row :type Name))
  (returns (List :type "Array of /Game/O_RPG/OpenRPG_Inventory/Structs/s_InventoryItem Structure"))
  (bind _returnvalue (`|GetDataTableRow` "/Game/O_RPG/OpenRPG_Inventory/Datatables/DT_ItemsList.DT_ItemsList" Row)
    (:`then`
      (return (`.Items_4_6695B8BB4D8D9B46DA7C12A393A152C4` (break `/Game/O_RPG/OpenRPG_Inventory/Structs/s_Loot` _returnvalue))))
    (:`RowNotFound`
      (return))))

(fn `GetPlayerInventory`
  (returns (PlayerInventory :type "/Game/O_RPG/OpenRPG_Inventory/Blueprints/Components/BPC_PlayerInventory Object Reference"))
  (return (`Actor.GetComponentByClass` (`GameplayStatics.GetPlayerCharacter` (`local.__WorldContext`)) "/Game/O_RPG/OpenRPG_Inventory/Blueprints/Components/BPC_PlayerInventory.BPC_PlayerInventory_C")))