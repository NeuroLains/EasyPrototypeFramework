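; Player inventory container component that adds money, item use, selling and interaction with nearby pickups, storage and shops.
; Slot clicks use items through actors spawned from their data class and cached per item, or quick-transfer to open storage or sell to an open shop when the modifier key is held.
; Slot drops route to rearranging, transfer or purchase by source container type.
; Save and load extend the parent's with money via the GameInstance.
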(event `self.Initialize`
  ;[0.03063 0.5441 1] Overrides the initialize event to update the inventory
  (`parent.Initialize`)
  (`self.UpdateContainerWidget`))

(event `self.OnSlotClicked`
  (params (ClickedIndex :type Integer))
  ;[1 0.03646 0.1158] Overriden event to use an item when a ui slot is clicked
  (if (`PlayerController.IsInputKeyDown` (`GameplayStatics.GetPlayerController` 0) (`self.QuickActionKey`))
    (`self.HandleQuickAction` ClickedIndex)
    (else
      (`self.UseItem` ClickedIndex))))

(event `UpdateMoney`
  (params (NewAmount :type Integer))
  ;[0.9946 1 0] UI Player Inventory Events
  (message `/Game/RPG/OpenRPG_Inventory/Blueprints/Interfaces/BPI_PlayerInventory.UpdateMoney` (`self.MainContainerWidget`) NewAmount))

(event `OpenStorage`
  (bind _nearbystorage (`self.NearbyStorage`))
  ;[0.1548 1 0.02316] Input events from player to use with interactables
  (`/Engine/EditorBlueprintResources/StandardMacros.IsValid` _nearbystorage
    (:`Is Valid`
      (message `/Game/RPG/OpenRPG_Inventory/Blueprints/Interfaces/BPI_WorldInteraction.OnInteract` _nearbystorage (`self.GetOwner`)))))

(event `OpenShop`
  (bind _nearbyshop (`self.NearbyShop`))
  ;[0.1548 1 0.02316] Input events from player to use with interactables
  (`/Engine/EditorBlueprintResources/StandardMacros.IsValid` _nearbyshop
    (:`Is Valid`
      (message `/Game/RPG/OpenRPG_Inventory/Blueprints/Interfaces/BPI_WorldInteraction.OnInteract` _nearbyshop (`self.GetOwner`)))))

(event `PickUpItem`
  (bind _output (`|GetArrayItem` (`self.NearbyItems`)))
  ;[0.1548 1 0.02316] Input events from player to use with interactables
  (`/Engine/EditorBlueprintResources/StandardMacros.IsValid` _output
    (:`Is Valid`
      (message `/Game/RPG/OpenRPG_Inventory/Blueprints/Interfaces/BPI_WorldInteraction.OnInteract` _output (`self.GetOwner`)))))

(fn `AddMoney`
  (params (Amount :type Integer))
  (returns (`Success?` :type Boolean))
  (locals (LocalAmount :type Integer) (LocalNewAmount :type Integer :default 0))
  (bind _output_get (set `local.LocalAmount` Amount))
  (bind _output_get_2 (set `local.LocalNewAmount` (+ _output_get (`self.CurrentMoney`))))
  (if (and (<= _output_get_2 (`self.MaxMoney`)) (>= (`local.LocalNewAmount`) 0))
    (bind _output_get_3 (set `self.CurrentMoney` (`local.LocalNewAmount`)))
    (`self.UpdateMoney` _output_get_3)
    (`self.OnMoneyAmountChanged` (`local.LocalAmount`) (`self.CurrentMoney`))
    (return true)
    (else
      (return false))))

(fn `AddNearbyItem`
  (params (NearbyActor :type "/Game/RPG/OpenRPG_Inventory/Blueprints/BP_WorldItem Object Reference"))
  (`KismetArrayLibrary.Array_AddUnique` (`self.NearbyItems`) NearbyActor)
  (return))

(fn `AddSpawnedActor`
  (params (Item :type Name) (Actor :type "/Game/RPG/OpenRPG_Inventory/Blueprints/BaseItemClasses/BP_BaseItem Object Reference"))
  (locals (LocalItem :type Name))
  (`BlueprintMapLibrary.Map_Add` (`self.SpawnedItems`) Item Actor)
  (return))

(fn `CanUseItem?`
  (params (Index :type Integer))
  (returns (`Success?` :type Boolean))
  (locals (LocalIndex :type Integer) (LocalPlayerLevel :type Integer :default 0))
  (set `local.LocalIndex` Index)
  (return (and (not (`self.IsSlotEmpty?` (`local.LocalIndex`))) (`.Usable?_78_5373B5A34DF8B45903FC91831E9FC4E8` (break `/Game/RPG/OpenRPG_Inventory/Structs/s_ItemData` (`/Game/RPG/OpenRPG_Inventory/Blueprints/Library/BPL_Inventory.GetItemDataByRow` (`.Item_8_78E0EFF340AA0567F5C6C3BC6148D1F0` (break `/Game/RPG/OpenRPG_Inventory/Structs/s_InventoryItem` (`self.GetItemAtIndex` (`local.LocalIndex`))))))))))

(fn `CreatePlayerSaveData`
  (returns (Data :type "/Game/RPG/OpenRPG_Inventory/Structs/s_PlayerInventorySaveData Structure"))
  (return (make `/Game/RPG/OpenRPG_Inventory/Structs/s_PlayerInventorySaveData` (`self.CurrentMoney`))))

(fn `HandleQuickAction`
  (params (ClickedIndex :type Integer))
  (locals (LocalClickedSlot :type Integer) (LocalStorage :type "/Game/RPG/OpenRPG_Inventory/Blueprints/Components/BPC_ItemsContainer Object Reference") (LocalShop :type "/Game/RPG/OpenRPG_Inventory/Blueprints/Components/BPC_ItemsContainer Object Reference"))
  (bind _returnvalue (`Actor.GetComponentByClass` (`self.NearbyShop`) "/Game/RPG/OpenRPG_Inventory/Blueprints/Components/BPC_ItemsContainer.BPC_ItemsContainer_C"))
  (bind _returnvalue_2 (`Actor.GetComponentByClass` (`self.NearbyStorage`) "/Game/RPG/OpenRPG_Inventory/Blueprints/Components/BPC_ItemsContainer.BPC_ItemsContainer_C"))
  (set `local.LocalClickedSlot` ClickedIndex)
  (if (`Widget.IsVisible` (`self.MainContainerWidget`))
    (`/Engine/EditorBlueprintResources/StandardMacros.IsValid` (`self.NearbyStorage`)
      (:`Is Valid`
        (`/Engine/EditorBlueprintResources/StandardMacros.IsValid` _returnvalue_2
          (:`Is Valid`
            (bind _output_get (set `local.LocalStorage` _returnvalue_2))
            (if (`Widget.IsVisible` (`/Game/RPG/OpenRPG_Inventory/Blueprints/Components/BPC_ItemsContainer.MainContainerWidget` _output_get))
              (`self.TransferItem` (`local.LocalStorage`) -1 (`local.LocalClickedSlot`))
              (return)
              (else
                (return))))
          (:`Is Not Valid`
            (return))))
      (:`Is Not Valid`
        (`/Engine/EditorBlueprintResources/StandardMacros.IsValid` (`self.NearbyShop`)
          (:`Is Valid`
            (`/Engine/EditorBlueprintResources/StandardMacros.IsValid` _returnvalue
              (:`Is Valid`
                (bind _output_get_2 (set `local.LocalShop` _returnvalue))
                (if (`Widget.IsVisible` (`/Game/RPG/OpenRPG_Inventory/Blueprints/Components/BPC_ItemsContainer.MainContainerWidget` _output_get_2))
                  (`self.SellItem` (`local.LocalClickedSlot`))
                  (return)
                  (else
                    (return))))
              (:`Is Not Valid`
                (return))))
          (:`Is Not Valid`
            (return)))))
    (else
      (return))))

(fn `HandleSlotDrop`
  (params (FromContainer :type "/Game/RPG/OpenRPG_Inventory/Blueprints/Components/BPC_ItemsContainer Object Reference") (FromIndex :type Integer) (DroppedIndex :type Integer))
  (locals (LocalFromContainer :type "/Game/RPG/OpenRPG_Inventory/Blueprints/Components/BPC_ItemsContainer Object Reference") (LocalFromIndex :type Integer) (LocalDroppedIndex :type Integer))
  (set `local.LocalFromContainer` FromContainer)
  (set `local.LocalFromIndex` FromIndex)
  (set `local.LocalDroppedIndex` DroppedIndex)
  (switch `/Game/RPG/OpenRPG_Inventory/Enums/e_ContainerType` (`/Game/RPG/OpenRPG_Inventory/Blueprints/Components/BPC_ItemsContainer.ContainerType` (`local.LocalFromContainer`))
    (:`NewEnumerator0`
      (`self.HandleSelfSlotDrop` (`local.LocalFromIndex`) (`local.LocalDroppedIndex`))
      (return))
    (:`NewEnumerator1`
      (`self.TransferItem` (`local.LocalFromContainer`) self (`local.LocalDroppedIndex`) (`local.LocalFromIndex`))
      (return))
    (:`NewEnumerator2`
      (`/Game/RPG/OpenRPG_Inventory/Blueprints/Components/BPC_Shop.BuyItem` (cast `/Game/RPG/OpenRPG_Inventory/Blueprints/Components/BPC_Shop` (`local.LocalFromContainer`) :!pure true) (`local.LocalFromIndex`) (`local.LocalDroppedIndex`))
      (return))))

(fn `LoadContainer`
  (params (SaveName :type String))
  (returns (`Sucsess?` :type Boolean))
  (locals (LocalSaveName :type String) (LocalPlayerData :type "/Game/RPG/OpenRPG_Inventory/Structs/s_PlayerInventorySaveData Structure"))
  (bind _output_get (set `local.LocalSaveName` SaveName))
  (bind _sucsess_ (`parent.LoadContainer` _output_get))
  (if _sucsess_
    (bind (_found_ _data) (message `/Game/RPG/OpenRPG_Inventory/Blueprints/Interfaces/BPI_PlayerInventorySave.LoadPlayerInventoryData` (`GameplayStatics.GetGameInstance`) (`local.LocalSaveName`)))
    (if _found_
      (bind _output_get_2 (set `local.LocalPlayerData` _data))
      (`self.AddMoney` (`.SavedMoney_2_56D7FFAB48EEAF6472A79591C75D579F` (break `/Game/RPG/OpenRPG_Inventory/Structs/s_PlayerInventorySaveData` _output_get_2)))
      (return true)
      (else
        (return false)))
    (else
      (return false))))

(fn `RemoveNearbyItem`
  (params (NearbyActor :type "/Game/RPG/OpenRPG_Inventory/Blueprints/BP_WorldItem Object Reference"))
  (`KismetArrayLibrary.Array_RemoveItem` (`self.NearbyItems`) NearbyActor)
  (return))

(fn `SaveContainer`
  (params (SaveName :type String) (`IsDiskSaveable?` :type Boolean))
  (returns (`Success?` :type Boolean))
  (locals (LocalSaveName :type String))
  (bind _output_get (set `local.LocalSaveName` SaveName))
  (bind _success_ (`parent.SaveContainer` _output_get `IsDiskSaveable?`))
  (if _success_
    (message `/Game/RPG/OpenRPG_Inventory/Blueprints/Interfaces/BPI_PlayerInventorySave.SavePlayerInventoryData` (`GameplayStatics.GetGameInstance`) (`local.LocalSaveName`) (`self.CreatePlayerSaveData`))
    (return true)
    (else
      (return false))))

(fn `SellItem`
  (params (Index :type Integer))
  (returns (`Success?` :type Boolean))
  (locals (LocalIndex :type Integer) (LocalItem :type Name) (LocalAmount :type Integer) (LocalBenefit :type Integer))
  (bind (_item _amount) (break `/Game/RPG/OpenRPG_Inventory/Structs/s_InventoryItem` (`self.GetItemAtIndex` (`local.LocalIndex`))))
  (bind ((`Type_13_957CA2D1456D6C9D4618728B02356F59` _type) (`Value_17_3EBC6C004B258E3102EC96B3560C9A5D` _value)) (break `/Game/RPG/OpenRPG_Inventory/Structs/s_ItemData` (`/Game/RPG/OpenRPG_Inventory/Blueprints/Library/BPL_Inventory.GetItemDataByRow` (`local.LocalItem`))))
  (set `local.LocalIndex` Index)
  (if (not (`self.IsSlotEmpty?` (`local.LocalIndex`)))
    (set `local.LocalItem` _item)
    (set `local.LocalAmount` _amount)
    (if (`|EnumInequality` _type "NewEnumerator2")
      (bind _output_get (set `local.LocalBenefit` (* _value (`local.LocalAmount`))))
      (bind _success_ (`self.AddMoney` _output_get))
      (if _success_
        (`self.RemoveIndexAmount` (`local.LocalIndex`) (`local.LocalAmount`))
        (return true)
        (else
          (return false)))
      (else
        (return false)))
    (else
      (return false))))

(fn `UseItem`
  (params (Index :type Integer))
  (returns (`Success?` :type Boolean))
  (locals (LocalIndex :type Integer) (LocalItemData :type "/Game/RPG/OpenRPG_Inventory/Structs/s_ItemData Structure") (LocalItemToUse :type "/Game/RPG/OpenRPG_Inventory/Blueprints/BaseItemClasses/BP_BaseItem Object Reference") (LocalItem :type Name))
  (bind _output_get (set `local.LocalIndex` Index))
  (if (`self.CanUseItem?` _output_get)
    (bind _output_get_2 (set `local.LocalItem` (`.Item_8_78E0EFF340AA0567F5C6C3BC6148D1F0` (break `/Game/RPG/OpenRPG_Inventory/Structs/s_InventoryItem` (`self.GetItemAtIndex` (`local.LocalIndex`))))))
    (bind _output_get_3 (set `local.LocalItemData` (`/Game/RPG/OpenRPG_Inventory/Blueprints/Library/BPL_Inventory.GetItemDataByRow` _output_get_2)))
    (if (`KismetSystemLibrary.IsValidClass` (`.Class_47_1920DEDC49E9F940C8E7B5830EF818FF` (break `/Game/RPG/OpenRPG_Inventory/Structs/s_ItemData` _output_get_3)))
      (bind _output_get_4 (set `local.LocalItemToUse` (`BlueprintMapLibrary.Map_Find` (`self.SpawnedItems`) (`local.LocalItem`))))
      (`/Engine/EditorBlueprintResources/StandardMacros.IsValid` _output_get_4
        (:`Is Valid`
          _)
        (:`Is Not Valid`
          (bind _returnvalue (`|SpawnActorFromClass` (`.Class_47_1920DEDC49E9F940C8E7B5830EF818FF` (break `/Game/RPG/OpenRPG_Inventory/Structs/s_ItemData` (`local.LocalItemData`))) (`KismetMathLibrary.MakeTransform` (0.0 0.0 0.0)) "AlwaysSpawn" "SelectDefaultAtRuntime" null (`local.LocalItem`) (`local.LocalItemData`) null)) ; This will spawn the class associated with the item that contains all the logic that has to be excuted
          (bind _output_get_5 (set `local.LocalItemToUse` _returnvalue))
          (`self.AddSpawnedActor` (`local.LocalItem`) _output_get_5)))
      (`/Game/RPG/OpenRPG_Inventory/Blueprints/BaseItemClasses/BP_BaseItem.UseItem` (`local.LocalItemToUse`) (`local.LocalIndex`)) ; Starts the item logic execution based on its type
      (`self.OnItemUsed` (`local.LocalItem`))
      (return true)
      (else
        (`self.OnItemUsed` (`local.LocalItem`))
        (return true)))
    (else
      (return false))))