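; BPC_Shop is the shop container component of the RPG inventory, handling buying and selling between the shop and the player.
; Clicking a slot calls BuyItem, which charges item value times amount from the player inventory, then adds the item to any slot or a given index.
; A failed add refunds the money, and insufficient funds prints a message.
; Dropping a player inventory item onto the shop sells it, while other drops are ignored.
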(event `self.OnSlotClicked`
  (params (ClickedIndex :type Integer))
  ;[1 0.03646 0.1158] Override On Slot Clicked: Just calls the function BuyItem
  (`self.BuyItem` ClickedIndex -1))

(fn `BuyItem`
  (params (Index :type Integer) (ToSpecificPlayerIndex :type Integer))
  (returns (Success :type Boolean))
  (locals (LocalIndex :type Integer) (LocalItemCost :type Integer) (LocalPlayerInventory :type "/Game/RPG/OpenRPG_Inventory/Blueprints/Components/BPC_PlayerInventory Object Reference") (LocalSpecificPlayerIndex :type Integer))
  (bind _localplayerinventory (`local.LocalPlayerInventory`))
  (bind _item (`self.GetItemAtIndex` (`local.LocalIndex`)))
  (bind (_item_2 _amount) (break `/Game/RPG/OpenRPG_Inventory/Structs/s_InventoryItem` (`self.GetItemAtIndex` (`local.LocalIndex`))))
  (set `local.LocalIndex` Index)
  (set `local.LocalSpecificPlayerIndex` ToSpecificPlayerIndex)
  (set `local.LocalItemCost` (* (`.Value_17_3EBC6C004B258E3102EC96B3560C9A5D` (break `/Game/RPG/OpenRPG_Inventory/Structs/s_ItemData` (`/Game/RPG/OpenRPG_Inventory/Blueprints/Library/BPL_Inventory.GetItemDataByRow` _item_2))) _amount))
  (bind _output_get (set `local.LocalPlayerInventory` (`/Game/RPG/OpenRPG_Inventory/Blueprints/Library/BPL_Inventory.GetPlayerInventory`)))
  (bind _success_ (`/Game/RPG/OpenRPG_Inventory/Blueprints/Components/BPC_PlayerInventory.AddMoney` _output_get (* (`local.LocalItemCost`) -1)))
  (if _success_
    (if (== (`local.LocalSpecificPlayerIndex`) -1)
      (bind _success__2 (`self.AddItem` _localplayerinventory _item))
      (if _success__2
        _
        (else
          (`/Game/RPG/OpenRPG_Inventory/Blueprints/Components/BPC_PlayerInventory.AddMoney` (`local.LocalPlayerInventory`) (`local.LocalItemCost`) :!label _label)
          (return false)))
      (else
        (bind _success__3 (`self.AddItemToIndex` _localplayerinventory _item (`local.LocalSpecificPlayerIndex`)))
        (if _success__3
          _
          (else
            (goto _label)))))
    (return true)
    (else
      (`KismetSystemLibrary.PrintString` "You dont have enough money to buy the item")
      (return false))))

(fn `HandleSlotDrop`
  (params (FromContainer :type "/Game/RPG/OpenRPG_Inventory/Blueprints/Components/BPC_ItemsContainer Object Reference") (FromIndex :type Integer) (DroppedIndex :type Integer))
  (locals (LocalFromContainer :type "/Game/RPG/OpenRPG_Inventory/Blueprints/Components/BPC_ItemsContainer Object Reference") (LocalFromIndex :type Integer) (LocalDroppedIndex :type Integer))
  (set `local.LocalFromContainer` FromContainer)
  (set `local.LocalFromIndex` FromIndex)
  (set `local.LocalDroppedIndex` DroppedIndex)
  (switch `/Game/RPG/OpenRPG_Inventory/Enums/e_ContainerType` (`/Game/RPG/OpenRPG_Inventory/Blueprints/Components/BPC_ItemsContainer.ContainerType` (`local.LocalFromContainer`))
    (:`NewEnumerator0`
      (`/Game/RPG/OpenRPG_Inventory/Blueprints/Components/BPC_PlayerInventory.SellItem` (cast `/Game/RPG/OpenRPG_Inventory/Blueprints/Components/BPC_PlayerInventory` (`local.LocalFromContainer`) :!pure true) (`local.LocalFromIndex`))
      (return))
    (:`NewEnumerator1`
      _)
    (:`NewEnumerator2`
      _))
  (return))