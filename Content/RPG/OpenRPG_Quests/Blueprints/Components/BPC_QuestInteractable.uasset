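; Quest component that tells an interactable actor which quest action it offers: finishing a quest, progressing a goal or accepting a quest.
; On BeginPlay it loads its quest and goal lists and a priority order from a data table row.
; It checks those lists against a passed-in quest manager in priority order, and UpdateQuestPriorityState broadcasts the first match with its quest ID.
; Add and remove functions edit the lists at runtime.
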(event `self.ReceiveBeginPlay`
  (`self.LoadTableData`))

(event `RefreshQuestInteractionState`
  (params (NewState :type "/Game/RPG/OpenRPG_Quests/Enums/e_QuestInteractionPriority Enum" :default "NewEnumerator0") (QuestID :type Name))
  (`self.OnQuestInteractionStateChanged` NewState QuestID))

(fn `AddGoalToProgress`
  (params (GoalID :type Name))
  (`KismetArrayLibrary.Array_AddUnique` (`self.GoalsToProgress`) GoalID)
  (return))

(fn `AddQuestToAccept`
  (params (QuestID :type Name))
  (`KismetArrayLibrary.Array_AddUnique` (`self.QuestsToAccept`) QuestID)
  (return))

(fn `AddQuestToFinish`
  (params (QuestID :type "Name (by ref)"))
  (`KismetArrayLibrary.Array_AddUnique` (`self.QuestsToFinish`) QuestID)
  (return))

(fn `CanAcceptQuest?`
  (params (QuestMananger :type "/Game/RPG/OpenRPG_Quests/Blueprints/Components/BPC_PlayerQuestManager Object Reference"))
  (returns (Out :type Boolean) (QuestID :type Name))
  (locals (LocalQuestManager :type "/Game/RPG/OpenRPG_Quests/Blueprints/Components/BPC_PlayerQuestManager Object Reference") (LocalQuest :type Name) (`LocalHasQuestToAccept?` :type Boolean))
  (set `local.LocalQuestManager` QuestMananger)
  (for _array_element (`self.QuestsToAccept`)
    (bind _output_get (set `local.LocalQuest` _array_element))
    (bind _output_get_2 (set `local.LocalHasQuestToAccept?` (`/Game/RPG/OpenRPG_Quests/Blueprints/Components/BPC_PlayerQuestManager.QuestCanBeAccepted?` (`local.LocalQuestManager`) _output_get)))
    (if _output_get_2
      (break)))
  (return (`local.LocalHasQuestToAccept?`) (`local.LocalQuest`)))

(fn `CanFinishQuest?`
  (params (QuestManager :type "/Game/RPG/OpenRPG_Quests/Blueprints/Components/BPC_PlayerQuestManager Object Reference"))
  (returns (Out :type Boolean) (QuestID :type Name))
  (locals (LocalQuestManager :type "/Game/RPG/OpenRPG_Quests/Blueprints/Components/BPC_PlayerQuestManager Object Reference") (LocalQuest :type Name) (`LocalHasFinisableQuest?` :type Boolean))
  (set `local.LocalQuestManager` QuestManager)
  (for _array_element (`self.QuestsToFinish`)
    (bind _output_get (set `local.LocalQuest` _array_element))
    (bind _output_get_2 (set `local.LocalHasFinisableQuest?` (`|EnumEquality` (`/Game/RPG/OpenRPG_Quests/Blueprints/Components/BPC_PlayerQuestManager.GetQuestState` (`local.LocalQuestManager`) _output_get) "NewEnumerator4")))
    (if _output_get_2
      (break)))
  (return (`local.LocalHasFinisableQuest?`) (`local.LocalQuest`)))

(fn `CanProgressGoal?`
  (params (QuestManager :type "/Game/RPG/OpenRPG_Quests/Blueprints/Components/BPC_PlayerQuestManager Object Reference"))
  (returns (Out :type Boolean) (Goal :type Name))
  (locals (LocalQuestManager :type "/Game/RPG/OpenRPG_Quests/Blueprints/Components/BPC_PlayerQuestManager Object Reference") (`HasGoalToProgress?` :type Boolean) (LocalGoal :type Name))
  (set `local.LocalQuestManager` QuestManager)
  (for _array_element (`self.GoalsToProgress`)
    (bind _output_get (set `local.LocalGoal` _array_element))
    (bind _output_get_2 (set `local.HasGoalToProgress?` (`/Game/RPG/OpenRPG_Quests/Blueprints/Components/BPC_PlayerQuestManager.IsGoalActive?` (`local.LocalQuestManager`) _output_get)))
    (if _output_get_2
      (break)))
  (return (`local.HasGoalToProgress?`) (`local.LocalGoal`)))

(fn `GetHighestPriorityQuestState`
  (params (QuestManager :type "/Game/RPG/OpenRPG_Quests/Blueprints/Components/BPC_PlayerQuestManager Object Reference"))
  (returns (PriorityState :type "/Game/RPG/OpenRPG_Quests/Enums/e_QuestInteractionPriority Enum") (QuestID :type Name) (GoalID :type Name))
  (locals (LocalQuestManager :type "/Game/RPG/OpenRPG_Quests/Blueprints/Components/BPC_PlayerQuestManager Object Reference") (LocalQuestPriority :type "/Game/RPG/OpenRPG_Quests/Enums/e_QuestInteractionPriority Enum" :default "NewEnumerator3") (LocalID :type Name))
  (bind (_out _questid) (`self.CanFinishQuest?` (`local.LocalQuestManager`)))
  (bind (_out_2 _questid_2) (`self.CanAcceptQuest?` (`local.LocalQuestManager`)))
  (bind (_out_3 _goal) (`self.CanProgressGoal?` (`local.LocalQuestManager`)))
  (set `local.LocalQuestManager` QuestManager)
  (for _array_element (`self.InteractionPriority`)
    (bind _output_get (set `local.LocalQuestPriority` _array_element))
    (switch `/Game/RPG/OpenRPG_Quests/Enums/e_QuestInteractionPriority` _output_get
      (:`NewEnumerator0`
        (if _out
          (set `local.LocalID` _questid)
          (break)))
      (:`NewEnumerator1`
        (if _out_3
          (set `local.LocalID` _goal)
          (break)))
      (:`NewEnumerator2`
        (if _out_2
          (set `local.LocalID` _questid_2)
          (break)))))
  (if (`|EnumEquality` (`local.LocalQuestPriority`) "NewEnumerator1")
    (return (`local.LocalQuestPriority`) (`/Game/RPG/OpenRPG_Quests/Blueprints/Components/BPC_PlayerQuestManager.GetQuestWithActiveGoal` (`local.LocalQuestManager`) (`local.LocalID`)) (`local.LocalID`))
    (else
      (return (`local.LocalQuestPriority`) (`local.LocalID`) "None"))))

(fn `LoadTableData`
  (`/Engine/EditorBlueprintResources/StandardMacros.IsValid` (`self.DataTable`)
    (:`Is Valid`
      (bind _returnvalue (`|GetDataTableRow` (`self.DataTable`) (`self.TableRow`))
        (:`then`
          (bind (_interactionpriority _queststoaccept _queststofinish _goalstocomplete) (break `/Game/RPG/OpenRPG_Quests/Structs/s_QuestInteractable` _returnvalue))
          (set `self.InteractionPriority` _interactionpriority)
          (set `self.QuestsToAccept` _queststoaccept)
          (set `self.QuestsToFinish` _queststofinish)
          (set `self.GoalsToProgress` _goalstocomplete)
          (return))
        (:`RowNotFound`
          (`self.PrintDebug` (`KismetStringLibrary.Concat_StrStr` "Row " (`KismetStringLibrary.Conv_NameToString` (`self.TableRow`)) " not found") (struct :`R` 1.0 :`G` 0.57707 :`A` 1.0) 10.0)
          (return))))
    (:`Is Not Valid`
      (`self.PrintDebug` "Datatable not valid in quest interactable component" (struct :`R` 1.0 :`G` 0.57707 :`A` 1.0) 10.0)
      (return))))

(fn `RemoveGoalToProgress`
  (params (GoalID :type Name))
  (`KismetArrayLibrary.Array_RemoveItem` (`self.GoalsToProgress`) GoalID)
  (return))

(fn `RemoveQuestToAccept`
  (params (QuestID :type Name))
  (`KismetArrayLibrary.Array_RemoveItem` (`self.QuestsToAccept`) QuestID)
  (return))

(fn `RemoveQuestToFinish`
  (params (QuestID :type Name))
  (`KismetArrayLibrary.Array_RemoveItem` (`self.QuestsToFinish`) QuestID)
  (return))

(fn `UpdateQuestPriorityState`
  (params (QuestManager :type "/Game/RPG/OpenRPG_Quests/Blueprints/Components/BPC_PlayerQuestManager Object Reference"))
  (locals (LocalQuestManager :type "/Game/RPG/OpenRPG_Quests/Blueprints/Components/BPC_PlayerQuestManager Object Reference"))
  (bind _output_get (set `local.LocalQuestManager` QuestManager))
  (bind (_prioritystate _questid) (`self.GetHighestPriorityQuestState` _output_get))
  (`self.RefreshQuestInteractionState` _prioritystate _questid)
  (return))