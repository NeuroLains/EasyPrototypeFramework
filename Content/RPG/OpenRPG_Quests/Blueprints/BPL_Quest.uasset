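; Blueprint function library of shared helpers for the RPG quest system.
; Finds player 0's quest manager component and uses its DataTable to look up static quest data by ID and required amounts for goals.
; Loads the quest save from a named slot, or creates a new, unsaved SaveQuestData object when none exists.
; Also maps quest states and categories to display colors.
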(fn `GetColorByQuestCategory`
  (params (QuestCategory :type "/Game/RPG/OpenRPG_Quests/Enums/e_QuestCategory Enum" :default "NewEnumerator0"))
  (returns (Color :type "LinearColor Structure"))
  (return (select `/Game/RPG/OpenRPG_Quests/Enums/e_QuestCategory` QuestCategory :`NewEnumerator0` (struct :`R` 0.953125 :`G` 0.939271 :`A` 1.0) :`NewEnumerator1` (struct :`G` 0.430671 :`B` 1.0 :`A` 1.0) :`NewEnumerator2` (struct :`R` 0.16064 :`G` 1.0 :`A` 1.0) :!type "LinearColor Structure")))

(fn `GetColorByQuestState`
  (params (State :type "/Game/RPG/OpenRPG_Quests/Enums/e_QuestState Enum" :default "NewEnumerator6"))
  (returns (Color :type "LinearColor Structure"))
  (return (select `/Game/RPG/OpenRPG_Quests/Enums/e_QuestState` State :`NewEnumerator6` (struct :`R` 0.28125 :`G` 0.28125 :`B` 0.28125 :`A` 1.0) :`NewEnumerator0` (struct :`R` 1.0 :`G` 1.0 :`B` 1.0 :`A` 1.0) :`NewEnumerator2` (struct :`R` 0.9375 :`A` 1.0) :`NewEnumerator4` (struct :`R` 0.019947 :`G` 0.9602 :`B` 1.0 :`A` 1.0) :`NewEnumerator5` (struct :`G` 1.0 :`B` 0.119515 :`A` 1.0) :!type "LinearColor Structure")))

(fn `GetPlayerQuestManagerComponent`
  (returns (PlayerQuestComponent :type "/Game/RPG/OpenRPG_Quests/Blueprints/Components/BPC_PlayerQuestManager Object Reference"))
  (return (`Actor.GetComponentByClass` (`GameplayStatics.GetPlayerCharacter` (`local.__WorldContext`)) "/Game/RPG/OpenRPG_Quests/Blueprints/Components/BPC_PlayerQuestManager.BPC_PlayerQuestManager_C")))

(fn `GetQuestGoalRequiredAmount`
  (params (QuestID :type Name) (GoalID :type Name))
  (returns (RequiredAmount :type Integer))
  (return (`.RequiredAmount_8_CD3DE141441C029A987C76894B1D3571` (break `/Game/RPG/OpenRPG_Quests/Structs/s_QuestGoal` (`BlueprintMapLibrary.Map_Find` (`.Goals_96_29D4306147187CDD8547C8BF9E5A5F6E` (break `/Game/RPG/OpenRPG_Quests/Structs/s_StaticQuestData` (`self.GetStaticQuestDataByID` QuestID))) GoalID)))))

(fn `GetQuestsSaveSlot`
  (params (SlotName :type String))
  (returns (SaveObject :type "/Game/RPG/OpenRPG_Quests/Blueprints/SaveQuestData Object Reference"))
  (locals (LocalSlotName :type String))
  (bind _output_get (set `local.LocalSlotName` SlotName))
  (bind _returnvalue (`GameplayStatics.DoesSaveGameExist` _output_get))
  (if _returnvalue
    (bind _returnvalue_2 (`GameplayStatics.LoadGameFromSlot` (`local.LocalSlotName`)))
    (bind _assave_quest_data (cast `/Game/RPG/OpenRPG_Quests/Blueprints/SaveQuestData` _returnvalue_2)
      (:`then`
        (return _assave_quest_data))
      (:`CastFailed`
        (return null)))
    (else
      (bind _returnvalue_3 (`GameplayStatics.CreateSaveGameObject` "/Game/RPG/OpenRPG_Quests/Blueprints/SaveQuestData.SaveQuestData_C"))
      (return _returnvalue_3))))

(fn `GetStaticQuestDataByID`
  (params (QuestID :type Name))
  (returns (StaticData :type "/Game/RPG/OpenRPG_Quests/Structs/s_StaticQuestData Structure"))
  (bind _datatable (`/Game/RPG/OpenRPG_Quests/Blueprints/Components/BPC_PlayerQuestManager.DataTable` (`self.GetPlayerQuestManagerComponent` (`local.__WorldContext`))))
  (`/Engine/EditorBlueprintResources/StandardMacros.IsValid` _datatable
    (:`Is Valid`
      (bind _returnvalue (`|GetDataTableRow` _datatable QuestID)
        (:`then`
          (return _returnvalue))
        (:`RowNotFound`
          _)))
    (:`Is Not Valid`
      _))
  (return))