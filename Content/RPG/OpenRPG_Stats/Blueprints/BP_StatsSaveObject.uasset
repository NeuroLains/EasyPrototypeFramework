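; Save object for the OpenRPG Stats system that holds stats, attributes and leveling data.
; Each category lives in its own map keyed by save name, written by a matching save event that adds or overwrites the entry.
; Matching load functions look up that name and return a found flag along with the stored data.
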(event `/Game/RPG/OpenRPG_Stats/Blueprints/Interfaces/BP_SaveLoad.SaveStats`
  (params (SaveName :type String) (Data :type "/Game/RPG/OpenRPG_Stats/Structs/s_StatsSaveData Structure"))
  (`BlueprintMapLibrary.Map_Add` (`self.SavedStatsData`) SaveName Data))

(event `/Game/RPG/OpenRPG_Stats/Blueprints/Interfaces/BP_SaveLoad.SaveAttributes`
  (params (SaveName :type String) (Data :type "/Game/RPG/OpenRPG_Stats/Structs/s_AttributesSaveData Structure"))
  (`BlueprintMapLibrary.Map_Add` (`self.SavedAttributesData`) SaveName Data))

(event `/Game/RPG/OpenRPG_Stats/Blueprints/Interfaces/BP_SaveLoad.SaveLeveling`
  (params (SaveName :type String) (Data :type "/Game/RPG/OpenRPG_Stats/Structs/s_LevelingSaveData Structure"))
  (`BlueprintMapLibrary.Map_Add` (`self.SavedLevelingData`) SaveName Data))

(fn `LoadAttributes`
  (params (SaveName :type String))
  (returns (`Found?` :type Boolean) (Data :type "/Game/RPG/OpenRPG_Stats/Structs/s_AttributesSaveData Structure"))
  (bind (_value _returnvalue) (`BlueprintMapLibrary.Map_Find` (`self.SavedAttributesData`) SaveName))
  (return _returnvalue _value))

(fn `LoadLeveling`
  (params (SaveName :type String))
  (returns (`Found?` :type Boolean) (Data :type "/Game/RPG/OpenRPG_Stats/Structs/s_LevelingSaveData Structure"))
  (bind (_value _returnvalue) (`BlueprintMapLibrary.Map_Find` (`self.SavedLevelingData`) SaveName))
  (return _returnvalue _value))

(fn `LoadStats`
  (params (SaveName :type String))
  (returns (`Found?` :type Boolean) (Data :type "/Game/RPG/OpenRPG_Stats/Structs/s_StatsSaveData Structure"))
  (bind (_value _returnvalue) (`BlueprintMapLibrary.Map_Find` (`self.SavedStatsData`) SaveName))
  (return _returnvalue _value))