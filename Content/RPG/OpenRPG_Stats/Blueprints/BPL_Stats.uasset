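; BPL_Stats is a Blueprint function library of shared helpers for the OpenRPG stats system.
; It fetches the stats, attributes and leveling components from player character 0.
; It looks up and validates buffs and effects by row name in DT_Buffs and DT_Effects, and substitutes the {value} token in effect descriptions.
; It also loads the stats save object from a fixed slot, creating an unsaved one if none exists.
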(fn `GetPlayerAttributesComponent`
  (returns (PlayerAttributes :type "/Game/RPG/OpenRPG_Stats/Blueprints/Components/BPC_Attributes Object Reference"))
  (return (`Actor.GetComponentByClass` (`GameplayStatics.GetPlayerCharacter` (`local.__WorldContext`)) "/Game/RPG/OpenRPG_Stats/Blueprints/Components/BPC_Attributes.BPC_Attributes_C")))

(fn `GetPlayerLevelingComponent`
  (returns (PlayerLeveling :type "/Game/RPG/OpenRPG_Stats/Blueprints/Components/BPC_Leveling Object Reference"))
  (return (`Actor.GetComponentByClass` (`GameplayStatics.GetPlayerCharacter` (`local.__WorldContext`)) "/Game/RPG/OpenRPG_Stats/Blueprints/Components/BPC_Leveling.BPC_Leveling_C")))

(fn `GetPlayerStatsComponent`
  (returns (PlayerStats :type "/Game/RPG/OpenRPG_Stats/Blueprints/Components/BPC_Stats Object Reference"))
  (return (`Actor.GetComponentByClass` (`GameplayStatics.GetPlayerCharacter` (`local.__WorldContext`)) "/Game/RPG/OpenRPG_Stats/Blueprints/Components/BPC_Stats.BPC_Stats_C")))

(fn `GetStaticBuffData`
  (params (Buff :type Name))
  (returns (Data :type "/Game/RPG/OpenRPG_Stats/Structs/s_BuffStatic Structure"))
  (bind _returnvalue (`|GetDataTableRow` "/Game/RPG/OpenRPG_Stats/Datatables/DT_Buffs.DT_Buffs" Buff)
    (:`then`
      (return _returnvalue))
    (:`RowNotFound`
      (return))))

(fn `GetStaticEffectData`
  (params (Effect :type Name))
  (returns (Data :type "/Game/RPG/OpenRPG_Stats/Structs/s_EffectStatic Structure"))
  (bind _returnvalue (`|GetDataTableRow` "/Game/RPG/OpenRPG_Stats/Datatables/DT_Effects.DT_Effects" Effect)
    (:`then`
      (return _returnvalue))
    (:`RowNotFound`
      (return))))

(fn `GetStatsSaveObject`
  (returns (SaveObject :type "/Game/RPG/OpenRPG_Stats/Blueprints/BP_StatsSaveObject Object Reference"))
  (locals (LocalSlotName :type String))
  (bind _output_get (set `local.LocalSlotName` (`self.GetStatsSlotName` (`local.__WorldContext`))))
  (bind _returnvalue (`GameplayStatics.DoesSaveGameExist` _output_get))
  (if _returnvalue
    (bind _returnvalue_2 (`GameplayStatics.LoadGameFromSlot` (`local.LocalSlotName`)))
    (bind _asbp_stats_save_object (cast `/Game/RPG/OpenRPG_Stats/Blueprints/BP_StatsSaveObject` _returnvalue_2)
      (:`then`
        (return _asbp_stats_save_object))
      (:`CastFailed`
        (return null)))
    (else
      (bind _returnvalue_3 (`GameplayStatics.CreateSaveGameObject` "/Game/RPG/OpenRPG_Stats/Blueprints/BP_StatsSaveObject.BP_StatsSaveObject_C"))
      (return _returnvalue_3))))

(fn `GetStatsSlotName`
  (returns (SlotName :type String))
  (return "OpenRPG_Stats"))

(fn `IsBuffValid?`
  (params (Buff :type Name))
  (returns (`Valid?` :type Boolean))
  (bind _returnvalue (`DataTableFunctionLibrary.DoesDataTableRowExist` "/Game/RPG/OpenRPG_Stats/Datatables/DT_Buffs.DT_Buffs" Buff))
  (return _returnvalue))

(fn `IsEffectValid?`
  (params (Effect :type Name))
  (returns (`Valid?` :type Boolean))
  (bind _returnvalue (`DataTableFunctionLibrary.DoesDataTableRowExist` "/Game/RPG/OpenRPG_Stats/Datatables/DT_Effects.DT_Effects" Effect))
  (return _returnvalue))

(fn `ParseEffectDescription`
  (params (Description :type Text) (Value :type "Float (double-precision)"))
  (returns (NewDescription :type Text))
  (return (`KismetTextLibrary.Conv_StringToText` (`KismetStringLibrary.Replace` (`KismetTextLibrary.Conv_TextToString` Description) "{value}" (`KismetStringLibrary.Conv_DoubleToString` Value)))))