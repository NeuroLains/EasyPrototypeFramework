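; Actor component that handles experience and leveling for its owner, configured from a data table row.
; Received experience carries over through repeated level-ups, each adding stat and attribute bonuses via sibling components and raising reward events.
; Experience thresholds come from the table or one of two formulas, with an optional debug consistency check.
; Registered widgets receive updates, and progress saves and loads through the GameInstance or a save slot.
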(event Custom|Initialize
  (Variables|Default|SetStatsComponent (Actor|GetComponentbyClass (Components|GetOwner) "/Game/RPG/OpenRPG_Stats/Blueprints/Components/BPC_Stats.BPC_Stats_C"))
  (Variables|Default|SetAttributesComponent (Actor|GetComponentbyClass (Components|GetOwner) "/Game/RPG/OpenRPG_Stats/Blueprints/Components/BPC_Attributes.BPC_Attributes_C"))
  (if (Variables|Settings|GetDebugEnabled?)
    (Consistency|CheckConsistency))
  (Save/Load|LoadTableData)
  (UI|RefreshWidgets))

(event Custom|UpdateLevel
  (params (NewLevel :type Integer))
  ;[0.06453 0.8803 1] Leveling
  (for _array_element (Variables|UI|GetWidgets)
    (Class|BPILeveling|UpdateDisplayedLevel(Message) _array_element NewLevel)))

(event Custom|UpdateExperience
  (params (CurrentExperience :type Integer) (NeededExperience :type Integer) (TotalExperience :type Integer))
  ;[0.06453 0.8803 1] Leveling
  (for _array_element (Variables|UI|GetWidgets)
    (Class|BPILeveling|UpdateDisplayedExperience(Message) _array_element CurrentExperience NeededExperience TotalExperience)))

(fn ReceiveExperience
  (params (Amount :type Integer))
  (LocalVariables|SetLocalReceivedAmount Amount)
  (if (< (Variables|General|GetCurrentLevel) (Variables|General|GetMaxLevel))
    (Variables|General|SetTotalExperience (+ (Variables|General|GetTotalExperience) (LocalVariables|GetLocalReceivedAmount)))
    (bind _output_get (Variables|General|SetCurrentExperience (+ (Variables|General|GetCurrentExperience) (LocalVariables|GetLocalReceivedAmount))))
    (while (and (>= _output_get (Variables|General|GetNeededExperience)) (< (Variables|General|GetCurrentLevel) (Variables|General|GetMaxLevel)))
      (Variables|General|SetCurrentExperience (- (Variables|General|GetCurrentExperience) (Variables|General|GetNeededExperience)))
      (Managment|LevelUp))
    (CallFunction|UpdateExperience (Variables|General|GetCurrentExperience) (Variables|General|GetNeededExperience) (Variables|General|GetTotalExperience))
    (Default|CallOnExperienceReceived (LocalVariables|GetLocalReceivedAmount) (Variables|General|GetCurrentExperience) (Variables|General|GetNeededExperience) (Variables|General|GetTotalExperience))
    (return)
    (else
      (return))))

(fn UpdateNeededExperience
  (bind _neededexperienceperlevel (Variables|General|GetNeededExperiencePerLevel))
  (bind _currentlevel (Variables|General|GetCurrentLevel))
  (bind (_value _returnvalue) (Utilities|Map|Find _neededexperienceperlevel _currentlevel))
  (if _returnvalue
    (Variables|General|SetNeededExperience _value)
    (return)
    (else
      (return))))

(fn LevelUp
  (bind _output_get (Variables|General|SetCurrentLevel (+ (Variables|General|GetCurrentLevel) 1)))
  (if (== _output_get (Variables|General|GetMaxLevel))
    _
    (else
      (Managment|UpdateNeededExperience)))
  (Managment|AddLevelBonuses)
  (Default|CallOnLevelUp (Variables|General|GetCurrentLevel))
  (if (.ReturnValue (Utilities|Map|Find (Utilities|Struct|Breaks_LevelingData (Managment|GetLevelingData)) (Variables|General|GetCurrentLevel)))
    (Default|CallOnReceiveLevelUpReward (Variables|General|GetCurrentLevel) (.Value (Utilities|Map|Find (Utilities|Struct|Breaks_LevelingData (Managment|GetLevelingData)) (Variables|General|GetCurrentLevel)))))
  (CallFunction|UpdateLevel (Variables|General|GetCurrentLevel))
  (return))

(fn RefreshWidgets
  (CallFunction|UpdateLevel (Variables|General|GetCurrentLevel))
  (CallFunction|UpdateExperience (Variables|General|GetCurrentExperience) (Variables|General|GetNeededExperience) (Variables|General|GetTotalExperience))
  (return))

(fn AddCustomWidgets
  (params (Widgets :type Array%20of%20User%20Widget%20Object%20References))
  (for _array_element Widgets
    (Utilities|Array|AddUnique (Variables|UI|GetWidgets) _array_element))
  (return))

(fn LoadTableData
  (Utilities|IsValid (Variables|Settings|GetLevelingTable)
    (:Is%20Valid
      (bind _output_get (LocalVariables|SetLocalLevelingData (Managment|GetLevelingData)))
      (Variables|General|SetStartingLevel (.StartingLevel (Utilities|Struct|Breaks_LevelingData _output_get)))
      (Variables|General|SetMaxLevel (.MaxLevel (Utilities|Struct|Breaks_LevelingData _output_get)))
      (Variables|General|SetNeededExperiencePerLevel (.NeededExperiencePerLevel (Utilities|Struct|Breaks_LevelingData _output_get)))
      (if (Utilities|Struct|Breaks_LevelingData (LocalVariables|GetLocalLevelingData))
        (Managment|CreateNeededExperiencebyFormula (Utilities|Struct|Breaks_LevelingData (LocalVariables|GetLocalLevelingData))))
      (if (Variables|Internal|GetHasLoadBeenSuccessful?)
        (return)
        (else
          (Variables|General|SetCurrentLevel (Variables|General|GetStartingLevel))
          (Managment|UpdateNeededExperience)
          (return))))
    (:Is%20Not%20Valid
      (return))))

(fn CreateSaveData
  (return (Utilities|Struct|Makes_LevelingSaveData (Variables|General|GetCurrentLevel) (Variables|General|GetCurrentExperience) (Variables|General|GetNeededExperience) (Variables|General|GetTotalExperience))))

(fn SaveData
  (params (SaveName :type String) (ToGameInstance? :type Boolean))
  (LocalVariables|SetLocalSaveName SaveName)
  (if ToGameInstance?
    (Class|BPSaveLoad|SaveLeveling(Message) (Game|GetGameInstance) (LocalVariables|GetLocalSaveName) (Save/Load|CreateSaveData))
    (return true)
    (else
      (bind _output_get (LocalVariables|SetLocalSaveObject (CallFunction|GetStatsSaveObject)))
      (Utilities|IsValid _output_get
        (:Is%20Valid
          (Class|BPSaveLoad|SaveLeveling(Message) (LocalVariables|GetLocalSaveObject) (LocalVariables|GetLocalSaveName) (Save/Load|CreateSaveData))
          (bind _returnvalue (SaveGame|SaveGametoSlot (LocalVariables|GetLocalSaveObject) (CallFunction|GetStatsSlotName)))
          (return _returnvalue))
        (:Is%20Not%20Valid
          (return false))))))

(fn LoadData
  (params (SaveName :type String) (FromGameInstance? :type Boolean))
  (LocalVariables|SetLocalSaveName SaveName)
  (if FromGameInstance?
    (bind (_found_ _data) (Class|BPSaveLoad|LoadLeveling(Message) (Game|GetGameInstance) (LocalVariables|GetLocalSaveName)))
    (if _found_
      (LocalVariables|SetLocalLevelingData _data)
      (else
        (return)))
    (else
      (bind _output_get (LocalVariables|SetLocalSaveObject (CallFunction|GetStatsSaveObject)))
      (Utilities|IsValid _output_get
        (:Is%20Valid
          (bind (_found__2 _data_2) (Class|BPSaveLoad|LoadLeveling(Message) (LocalVariables|GetLocalSaveObject) (LocalVariables|GetLocalSaveName)))
          (if _found__2
            (LocalVariables|SetLocalLevelingData _data_2)
            (else
              (return))))
        (:Is%20Not%20Valid
          (return)))))
  (Variables|General|SetCurrentLevel (.CurrentLevel (Utilities|Struct|Breaks_LevelingSaveData (LocalVariables|GetLocalLevelingData))))
  (Variables|General|SetCurrentExperience (.CurrentExperience (Utilities|Struct|Breaks_LevelingSaveData (LocalVariables|GetLocalLevelingData))))
  (Variables|General|SetNeededExperience (.NeededExperience (Utilities|Struct|Breaks_LevelingSaveData (LocalVariables|GetLocalLevelingData))))
  (Variables|General|SetTotalExperience (.TotalExperience (Utilities|Struct|Breaks_LevelingSaveData (LocalVariables|GetLocalLevelingData))))
  (Variables|Internal|SetHasLoadBeenSuccessful? true)
  (return))

(fn ApplyExperienceFormula
  (params (Level :type Integer) (FormulaType :type e_ExperienceFormulaType%20Enum :default "NewEnumerator0"))
  (LocalVariables|SetLocalLevel Level)
  (switch Utilities|FlowControl|Switch|Switchone_ExperienceFormulaType FormulaType
    (:NewEnumerator0
      (if (!= (LocalVariables|GetLocalLevel) (Variables|General|GetStartingLevel))
        (return (Math|Float|Truncate (|(a+(b*100)) (Math|Conversions|ToFloat(Integer) (.Value (Utilities|Map|Find (Variables|General|GetNeededExperiencePerLevel) (Variables|General|GetStartingLevel)))) (Math|Conversions|ToFloat(Integer) (LocalVariables|GetLocalLevel)))))
        (else
          (return (.Value (Utilities|Map|Find (Variables|General|GetNeededExperiencePerLevel) (Variables|General|GetStartingLevel)))))))
    (:NewEnumerator1
      (return (Math|Float|Truncate (|(a+(a*0.100000)) (Math|Conversions|ToFloat(Integer) (.Value (Utilities|Map|Find (Variables|General|GetNeededExperiencePerLevel) (- (LocalVariables|GetLocalLevel) 1))))))))))

(fn CheckConsistency
  (Utilities|IsValid (Variables|Settings|GetLevelingTable)
    (:Is%20Valid
      (bind _returnvalue (Utilities|GetDataTableRow (Variables|Settings|GetLevelingTable) (Variables|Settings|GetLevelingTableRow))
        (:then
          (bind _output_get (LocalVariables|SetLocalLevelingData _returnvalue))
          (if (Utilities|Struct|Breaks_LevelingData _output_get)
            (Development|PrintString "No errors found!" true false "(R=0.000000,G=1.000000,B=0.000000,A=1.000000)" 5.0)
            (return)
            (else
              (for _index (range (.StartingLevel (Utilities|Struct|Breaks_LevelingData (LocalVariables|GetLocalLevelingData))) (.MaxLevel (Utilities|Struct|Breaks_LevelingData (LocalVariables|GetLocalLevelingData))))
                (bind _output_get_2 (LocalVariables|SetLocalLevel _index))
                (if (not (Utilities|Map|Contains (Utilities|Struct|Breaks_LevelingData (LocalVariables|GetLocalLevelingData)) _output_get_2))
                  (Development|PrintString (Utilities|String|Append "Error: You are not using experience formula and level  " (Utilities|String|ToString(Integer) (LocalVariables|GetLocalLevel)) " wasnt found in NeededExperiencePerLevel, if you reach that level system wont assign NeededExperience properly!") true false "(R=1.000000,G=0.000000,B=0.000000,A=1.000000)" 1e+01)
                  (return)))
              (Development|PrintString "No errors found!" true false "(R=0.000000,G=1.000000,B=0.000000,A=1.000000)" 5.0)
              (return))))
        (:RowNotFound
          (Development|PrintString (Utilities|String|Append "LevelingTableRow " (Utilities|String|ToString(Name) (Variables|Settings|GetLevelingTableRow)) " not found in LevelingTable") true false "(R=1.000000,G=0.000000,B=0.000000,A=1.000000)" 1e+01)
          (return))))
    (:Is%20Not%20Valid
      (Development|PrintString "Error: Not valid AttributesTable value assigned" true false "(R=1.000000,G=0.000000,B=0.000000,A=1.000000)" 1e+01)
      (return))))

(fn CreateNeededExperiencebyFormula
  (params (Formula :type e_ExperienceFormulaType%20Enum :default "NewEnumerator0"))
  (LocalVariables|SetLocalFormula Formula)
  (for _index (range (Variables|General|GetStartingLevel) (Variables|General|GetMaxLevel))
    (Utilities|Map|Add (Variables|General|GetNeededExperiencePerLevel) _index (Managment|ApplyExperienceFormula _index (LocalVariables|GetLocalFormula))))
  (return))

(fn GetLevelingData
  (bind _returnvalue (Utilities|GetDataTableRow (Variables|Settings|GetLevelingTable) (Variables|Settings|GetLevelingTableRow))
    (:then
      (return _returnvalue))
    (:RowNotFound
      (return ""))))

(fn AddLevelBonuses
  (bind _attributescomponent (Variables|Default|GetAttributesComponent)
    (:then
      (Default|AddAttributesPerLevel _attributescomponent))
    (:else
      _))
  (bind _statscomponent (Variables|Default|GetStatsComponent)
    (:then
      (Default|AddStatsPerLevel _statscomponent))
    (:else
      _))
  (return))