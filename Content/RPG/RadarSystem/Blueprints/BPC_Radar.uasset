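; Player component that drives a horizontal compass radar (WB_Radar) showing directions and BPI_Marker actors with distance and elevation arrows.
; Markers come from a world scan, ID, actor or spawned location.
; Yaw deltas from the camera, scaled by field of view, become widget offsets, with off-sight markers hidden or pinned to the edge.
; Turn and move inputs drive updates, while Tick runs only for movable markers or jumps to save performance.
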(event `Initialize`
  (params (PlayerCamera :type "CameraComponent Object Reference"))
  ;[1 0.0478 0.2078] Initializes the radar, it needs the camera as input
  (set `self.PlayerCamera` PlayerCamera)
  (set `self.Player` (`self.GetOwner`))
  (bind _foundwidgets (`WidgetBlueprintLibrary.GetAllWidgetsOfClass` "/Game/RPG/RadarSystem/Widgets/WB_Radar.WB_Radar_C" false))
  (bind _output_get (set `self.RadarWidget` (`|GetArrayItem` _foundwidgets)))
  (`/Engine/EditorBlueprintResources/StandardMacros.IsValid` _output_get
    (:`Is Valid`
      (`self.AddDirectionWidgets`)
      (`self.ScanWorldMarkers`)
      (set `self.MaxWidgetTranslation` (/ (`/Game/RPG/RadarSystem/Widgets/WB_Radar.GetRadarWidth` (`self.RadarWidget`)) 2.0)))))

(event `UpdatePlayerCamera`
  (params (Camera :type "CameraComponent Object Reference"))
  ;[1 0.9714 0.1763] Updates the player camera with a new one
  (set `self.PlayerCamera` Camera))

(event `UpdatePlayerTurnAxis`
  (params (AxisValue :type "Float (double-precision)"))
  ;[0.1354 0.684 1] Updates the player turn axis, so we know if we need to update the directions and the marker positions
  (bind _output_get (set `self.PlayerTurnAxisValue` AxisValue))
  (bind _output_get_2 (set `self.IsPlayerTurning?` (!= _output_get 0.0)))
  (if (and _output_get_2 (`Widget.IsVisible` (`self.RadarWidget`)))
    (`self.UpdateDirections`)
    (if (not (`self.IsPlayerMoving?`))
      (`self.UpdateMarkerPositions` false))))

(event `UpdatePlayerForwardAxisValue`
  (params (AxisValue :type "Float (double-precision)"))
  ;[0.1354 0.684 1] Updates the player move forward and move right axis, it will be useful to know when to update the markers
  (set `self.PlayerForwardAxisValue` AxisValue)
  (bind _output_get (set `self.IsPlayerMoving?` (or (!= (`self.PlayerForwardAxisValue`) 0.0) (!= (`self.PlayerRightAxisValue`) 0.0)) :!label _label))
  (if (and _output_get (`Widget.IsVisible` (`self.RadarWidget`)))
    (`self.UpdateMarkers` false)))

(event `UpdatePlayerRightAxisValue`
  (params (AxisValue :type "Float (double-precision)"))
  ;[0.1354 0.684 1] Updates the player move forward and move right axis, it will be useful to know when to update the markers
  (set `self.PlayerRightAxisValue` AxisValue)
  (goto _label))

(event `OnPlayerJumps`
  ;[0.07908 0.1965 1] Event that handles the radar updating while the player is jumping, because if the player is in the air and the is no movement key pressed, the radar wouldnt update
  (set `self.IsPlayerJumping?` true)
  (`self.SetComponentTickEnabled` true))

(event `self.ReceiveTick`
  (params (DeltaSeconds :type "Float (single-precision)"))
  ;[0.2865 1 0.01465] Event tick is disabled by default to get the best performance. It will be enabled only when there is a movable marker in the radar, so if it moves but the player doesnt, the marker movement will be visible in the radar
  (if (and (`Widget.IsVisible` (`self.RadarWidget`)) (not (`self.IsPlayerMoving?`)))
    (if (`self.IsPlayerJumping?`)
      (`self.UpdateMarkers` false)
      (if (not (`NavMovementComponent.IsFalling` (`Actor.GetComponentByClass` (`self.Player`) "/Script/Engine.CharacterMovementComponent")))
        (set `self.IsPlayerJumping?` false)
        (`self.SetComponentTickEnabled` (> (`self.MovableMarkersCount`) 0)))
      (else
        (`self.UpdateMarkers` true)))))

(event `OnNearbyHighLightActorsAmountChange`
  (params (NewAmount :type Integer))
  (`/Game/RPG/RadarSystem/Widgets/WB_Radar.OnNearbyHighLightActorsAmountChanged` (`self.RadarWidget`) NewAmount))

(event `AddDirectionWidget`
  (params (Direction :type Name))
  (`/Game/RPG/RadarSystem/Widgets/WB_Radar.AddDirection` (`self.RadarWidget`) Direction))

(event `AddMarkerWidget`
  (params (Marker :type "/Game/RPG/RadarSystem/Structs/s_MarkerTypeData Structure"))
  (`/Game/RPG/RadarSystem/Widgets/WB_Radar.AddMarker` (`self.RadarWidget`) Marker))

(event `UpdateDirectionPosition`
  (params (Direction :type Name) (NewPosition :type "Vector2D Structure") (`OnRadarSight?` :type Boolean))
  (`/Game/RPG/RadarSystem/Widgets/WB_Radar.UpdateDirectionPosition` (`self.RadarWidget`) Direction NewPosition `OnRadarSight?`))

(event `UpdateMarkerPosition`
  (params (MarkerIndex :type Integer) (NewPosition :type "Vector2D Structure") (`OnRadarSight?` :type Boolean) (`Hide?` :type Boolean))
  (`/Game/RPG/RadarSystem/Widgets/WB_Radar.UpdateMarkerPosition` (`self.RadarWidget`) MarkerIndex NewPosition `OnRadarSight?` `Hide?`))

(event `UpdateMarkerDistance`
  (params (MarkerIndex :type Integer) (NewDistance :type "Float (double-precision)"))
  (`/Game/RPG/RadarSystem/Widgets/WB_Radar.UpdateMarkerDistance` (`self.RadarWidget`) MarkerIndex NewDistance))

(event `UpdateMarkerElevationArrow`
  (params (MarkerIndex :type Integer) (`Up?` :type Boolean) (Hide :type Boolean))
  (`/Game/RPG/RadarSystem/Widgets/WB_Radar.UpdateMarkerElevationArrow` (`self.RadarWidget`) MarkerIndex `Up?` Hide))

(event `RemoveMarkerWidget`
  (params (Index :type Integer))
  (`/Game/RPG/RadarSystem/Widgets/WB_Radar.RemoveMarker` (`self.RadarWidget`) Index))

(fn `AddActorMarker`
  (params (Actor :type "Actor Object Reference"))
  (locals (LocalActor :type "Actor Object Reference") (LocalMarkerType :type Name :default "None") (`LocalMovable?` :type Boolean :default false) (LocalMarkerStaticData :type "/Game/RPG/RadarSystem/Structs/s_MarkerTypeData Structure") (LocalID :type Name :default "None"))
  (bind _output_get (set `local.LocalActor` Actor))
  (`/Engine/EditorBlueprintResources/StandardMacros.IsValid` _output_get
    (:`Is Valid`
      (if (`KismetSystemLibrary.DoesImplementInterface` (`local.LocalActor`) "/Game/RPG/RadarSystem/Blueprints/BPI_Marker.BPI_Marker_C")
        (if (not (`self.IsActorBeingTracked?` (`local.LocalActor`)))
          (bind (_id _markertype _movable_) (message `/Game/RPG/RadarSystem/Blueprints/BPI_Marker.GetMarkerData` (`local.LocalActor`)))
          (set `local.LocalID` _id)
          (set `local.LocalMarkerType` _markertype)
          (set `local.LocalMovable?` _movable_)
          (set `local.LocalMarkerStaticData` (`/Game/RPG/RadarSystem/Blueprints/BPL_Radar.GetMarkerTypeData` (`local.LocalMarkerType`)))
          (`KismetArrayLibrary.Array_Add` (`self.Markers`) (make `/Game/RPG/RadarSystem/Structs/s_DynamicMarker` (`local.LocalID`) (`local.LocalMarkerType`) (`local.LocalMarkerStaticData`) (`local.LocalActor`) (`local.LocalMovable?`)))
          (`self.AddMarkerWidget` (`local.LocalMarkerStaticData`))
          (`self.UpdateMarkers` false)
          (if (`local.LocalMovable?`)
            (bind _output_get_2 (set `self.MovableMarkersCount` (+ (`self.MovableMarkersCount`) 1)))
            (`self.SetComponentTickEnabled` (> _output_get_2 0))
            (return)
            (else
              (return)))
          (else
            (return)))
        (else
          (return))))
    (:`Is Not Valid`
      (return))))

(fn `AddDirectionWidgets`
  (bind _keys (`BlueprintMapLibrary.Map_Keys` (`self.Directions`)))
  (for _array_element _keys
    (`self.AddDirectionWidget` _array_element)))

(fn `AddHighLightActor`
  (params (Actor :type "Actor Object Reference"))
  (locals (LocalActor :type "Actor Object Reference"))
  (bind _output_get (set `local.LocalActor` Actor))
  (`/Engine/EditorBlueprintResources/StandardMacros.IsValid` _output_get
    (:`Is Valid`
      (`KismetArrayLibrary.Array_AddUnique` (`self.NearbyHighLightActors`) (`local.LocalActor`))
      (`self.OnNearbyHighLightActorsAmountChange` (`KismetArrayLibrary.Array_Length` (`self.NearbyHighLightActors`)))
      (return))
    (:`Is Not Valid`
      (return))))

(fn `AddLocationMarker`
  (params (SpawnLocation :type "Vector Structure") (MarkerType :type Name))
  (returns (SpawnedWorldMarker :type "Actor Object Reference"))
  (locals (LocalSpawnedWorldMarker :type "/Game/RPG/RadarSystem/Blueprints/BP_RadarWorldMarker Object Reference") (LocalMarkerType :type Name))
  (bind _returnvalue (`|SpawnActorFromClass` "/Game/RPG/RadarSystem/Blueprints/BP_RadarWorldMarker.BP_RadarWorldMarker_C" (`KismetMathLibrary.MakeTransform` SpawnLocation) "Undefined" "OverrideRootScale" null MarkerType null))
  (bind _output_get (set `local.LocalSpawnedWorldMarker` _returnvalue))
  (`self.AddActorMarker` _output_get)
  (return (`local.LocalSpawnedWorldMarker`)))

(fn `AddMarkersByID`
  (params (ID :type "Array of Name"))
  (locals (LocalIDs :type "Array of Name"))
  (set `local.LocalIDs` ID)
  (bind _outactors (`GameplayStatics.GetAllActorsWithInterface` "/Game/RPG/RadarSystem/Blueprints/BPI_Marker.BPI_Marker_C"))
  (for _array_element _outactors
    (bind _id (message `/Game/RPG/RadarSystem/Blueprints/BPI_Marker.GetMarkerData` _array_element))
    (if (`KismetArrayLibrary.Array_Contains` (`local.LocalIDs`) _id)
      (`self.AddActorMarker` _array_element)))
  (return))

(fn `CalculateMarkerArrow`
  (params (Actor :type "Actor Object Reference"))
  (returns (`Up?` :type Boolean) (`Hide?` :type Boolean))
  (locals (LocalHeightDifference :type "Float (double-precision)" :default 0.0))
  (bind _output_get (set `local.LocalHeightDifference` (`/Game/RPG/RadarSystem/Blueprints/BPL_Radar.ConvertUnrealUnitsToMetric` (`self.Metric`) (- (.z (`Actor.K2_GetActorLocation` Actor)) (.z (`Actor.K2_GetActorLocation` (`self.Player`)))))))
  (return (> _output_get 0.0) (< (`KismetMathLibrary.Abs` _output_get) (`self.ArrowHeightRange`))))

(fn `CalculateTranslation`
  (params (TargetDirection :type "Vector Structure"))
  (returns (Translation :type "Vector2D Structure") (`InRadarSight?` :type Boolean))
  (locals (LocalTarget :type "Vector Structure") (LocalTargetDirection :type "Vector Structure" :default (0.0 0.0 0.0)) (LocalForwardDotProduct :type "Float (double-precision)" :default 0.0) (LocalRightDotProduct :type "Float (double-precision)" :default 0.0) (LocalIsInRightSideOfRadar :type Boolean :default false) (`LocalIsDirection?` :type Boolean))
  (bind (_returnvalue_roll _returnvalue_pitch _returnvalue_yaw) (`KismetMathLibrary.BreakRotator` (`SceneComponent.K2_GetComponentRotation` (`self.PlayerCamera`))))
  (set `local.LocalTargetDirection` TargetDirection)
  ;[0.07192 0.3039 1] Calculates the dot product between two vectors. One of them is the direction we are targeting with the camera, and the another one is the vector that goes from the player to the marker
  (set `local.LocalForwardDotProduct` (`KismetMathLibrary.Dot_VectorVector` (`self.ConvertWorldRotationToUnitVector` _returnvalue_yaw) (`local.LocalTargetDirection`)))
  ;[0.1407 0.5617 1] We again use the dot product with the right vector to the camera to check the side of the radar widget to translate the marker
  (bind _output_get (set `local.LocalRightDotProduct` (`KismetMathLibrary.Dot_VectorVector` (`SceneComponent.GetRightVector` (`self.PlayerCamera`)) (`local.LocalTargetDirection`))))
  (set `local.LocalIsInRightSideOfRadar` (>= _output_get 0.0))
  ;[1 0.03119 0.04114] If true it means we can see the marker, false means opposite
  (if (>= (`local.LocalForwardDotProduct`) 0.0)
    (return (`KismetMathLibrary.MakeVector2D` (* (* (`self.MaxWidgetTranslation`) (- 1.0 (`local.LocalForwardDotProduct`))) (`KismetMathLibrary.SelectFloat` 1.0 -1.0 (`local.LocalIsInRightSideOfRadar`)))) true)
    (else
      (return (`KismetMathLibrary.MakeVector2D` (* (`self.MaxWidgetTranslation`) (`KismetMathLibrary.SelectFloat` 1.0 -1.0 (`local.LocalIsInRightSideOfRadar`)))) false))))

(fn `ConvertRotationToCircleDegrees`
  (params (Rotation :type "Float (double-precision)"))
  (returns (CircleDegrees :type "Float (double-precision)"))
  (locals (LocalRotation :type "Float (double-precision)"))
  (bind _output_get (set `local.LocalRotation` Rotation))
  (return (mod (`KismetMathLibrary.SelectFloat` _output_get (+ (`local.LocalRotation`) 360.0) (>= (`local.LocalRotation`) 0.0)) 360.0)))

(fn `ConvertRotationToTranslation`
  (params (`Rotation A` :type "Rotator Structure") (`Rotation B` :type "Rotator Structure"))
  (returns (Translation :type "Vector2D Structure") (`Clockwise?` :type Boolean) (`OnRadarSight?` :type Boolean))
  (locals (LocalClockwiseDelta :type "Float (double-precision)" :default 0.0) (LocalAntiClockwiseDelta :type "Float (double-precision)" :default 0.0))
  (bind _circledegrees (`self.ConvertRotationToCircleDegrees` (.yaw `Rotation B`)))
  (bind _circledegrees_2 (`self.ConvertRotationToCircleDegrees` (.yaw `Rotation A`)))
  (bind _returnvalue (/ (`local.LocalAntiClockwiseDelta`) (`CameraComponent.FieldOfView` (`self.PlayerCamera`))))
  (bind _returnvalue_2 (/ (`local.LocalClockwiseDelta`) (`CameraComponent.FieldOfView` (`self.PlayerCamera`))))
  (set `local.LocalClockwiseDelta` (`self.GetDeltaDegrees` _circledegrees_2 _circledegrees true))
  (set `local.LocalAntiClockwiseDelta` (`self.GetDeltaDegrees` _circledegrees_2 _circledegrees))
  (`/Engine/EditorBlueprintResources/StandardMacros.CompareFloat` (`local.LocalClockwiseDelta`) (`local.LocalAntiClockwiseDelta`)
    (:`>`
      (if (<= _returnvalue 1.0)
        (return (`KismetMathLibrary.MakeVector2D` (* (`KismetMathLibrary.Lerp` 0.0 (`self.MaxWidgetTranslation`) _returnvalue) -1.0)) false true)
        (else
          (return (0.0 0.0) false false))))
    (:`==`
      _)
    (:`<`
      _))
  (if (<= _returnvalue_2 1.0)
    (return (`KismetMathLibrary.MakeVector2D` (`KismetMathLibrary.Lerp` 0.0 (`self.MaxWidgetTranslation`) _returnvalue_2)) true true)
    (else
      (return (0.0 0.0) true false))))

(fn `ConvertWorldRotationToUnitVector`
  (params (WorldRotation :type "Float (double-precision)"))
  (returns (Vector :type "Vector Structure"))
  ;[0.5068 1 0.1131] This function converts an angle to a unit vector
  (return (`KismetMathLibrary.MakeVector` (`KismetMathLibrary.DegCos` WorldRotation) (`KismetMathLibrary.DegSin` WorldRotation))))

(fn `GetDeltaDegrees`
  (params (A :type "Float (double-precision)") (B :type "Float (double-precision)") (`Clockwise?` :type Boolean))
  (returns (Delta :type "Float (double-precision)"))
  (locals (LocalA :type "Float (double-precision)") (LocalB :type "Float (double-precision)"))
  (bind _locala (`local.LocalA`))
  (set `local.LocalA` A)
  (set `local.LocalB` B)
  (if `Clockwise?`
    (`/Engine/EditorBlueprintResources/StandardMacros.CompareFloat` (`local.LocalA`) (`local.LocalB`)
      (:`>`
        (return (- 360.0 (- (`local.LocalA`) (`local.LocalB`)))))
      (:`==`
        (return 0.0))
      (:`<`
        (return (- (`local.LocalB`) _locala))))
    (else
      (`/Engine/EditorBlueprintResources/StandardMacros.CompareFloat` (`local.LocalA`) (`local.LocalB`)
        (:`>`
          (return (- _locala (`local.LocalB`))))
        (:`==`
          (return 0.0))
        (:`<`
          (return (- 360.0 (- (`local.LocalB`) (`local.LocalA`)))))))))

(fn `IsActorBeingTracked?`
  (params (Actor :type "Actor Object Reference"))
  (returns (`Tracked?` :type Boolean))
  (locals (LocalActor :type "Actor Object Reference") (`LocalTracked?` :type Boolean))
  (set `local.LocalActor` Actor)
  (for _array_element (`self.Markers`)
    (bind _output_get (set `local.LocalTracked?` (== (`.AttachedActor_6_584AF733497E0D1B9A2C08AB05C24118` (break `/Game/RPG/RadarSystem/Structs/s_DynamicMarker` _array_element)) (`local.LocalActor`))))
    (if _output_get
      (break)))
  (return (`local.LocalTracked?`)))

(fn `IsActorMoving?`
  (params (Actor :type "Actor Object Reference"))
  (returns (`Moving?` :type Boolean))
  (return (> (`KismetMathLibrary.VSize` (`Actor.GetVelocity` Actor)) 0.0)))

(fn `RemoveHighLightActor`
  (params (Actor :type "Actor Object Reference"))
  (locals (LocalActor :type "Actor Object Reference"))
  (bind _output_get (set `local.LocalActor` Actor))
  (`/Engine/EditorBlueprintResources/StandardMacros.IsValid` _output_get
    (:`Is Valid`
      (`KismetArrayLibrary.Array_RemoveItem` (`self.NearbyHighLightActors`) (`local.LocalActor`))
      (`self.OnNearbyHighLightActorsAmountChange` (`KismetArrayLibrary.Array_Length` (`self.NearbyHighLightActors`)))
      (return))
    (:`Is Not Valid`
      (return))))

(fn `RemoveMarker`
  (params (MarkerIndex :type Integer))
  (locals (LocalMarkerIndex :type Integer))
  (bind _localmarkerindex (`local.LocalMarkerIndex`))
  (bind _output_get (set `local.LocalMarkerIndex` MarkerIndex))
  (if (`.IsMovable?_13_651DF0D84FAABF37F1ED1AA6758E1C88` (break `/Game/RPG/RadarSystem/Structs/s_DynamicMarker` (`|GetArrayItem` (`self.Markers`) _output_get)))
    (bind _output_get_2 (set `self.MovableMarkersCount` (- (`self.MovableMarkersCount`) 1)))
    (`self.SetComponentTickEnabled` (> _output_get_2 0)))
  (`KismetArrayLibrary.Array_Remove` (`self.Markers`) _localmarkerindex)
  (`self.RemoveMarkerWidget` _localmarkerindex)
  (return))

(fn `RemoveMarkerByAttachedActor`
  (params (Actor :type "Actor Object Reference"))
  (locals (LocalActor :type "Actor Object Reference"))
  (set `local.LocalActor` Actor)
  (bind (_arrayindex _arrayelement) (`/Engine/EditorBlueprintResources/StandardMacros.ReverseForEachLoop` (`self.Markers`))
    (:`LoopBody`
      (if (== (`.AttachedActor_6_584AF733497E0D1B9A2C08AB05C24118` (break `/Game/RPG/RadarSystem/Structs/s_DynamicMarker` _arrayelement)) (`local.LocalActor`))
        (`self.RemoveMarker` _arrayindex)
        (return)))
    (:`Completed`
      (return))))

(fn `RemoveMarkersByID`
  (params (ID :type Name))
  (locals (LocalID :type Name))
  (set `local.LocalID` ID)
  (bind (_arrayindex _arrayelement) (`/Engine/EditorBlueprintResources/StandardMacros.ReverseForEachLoop` (`self.Markers`))
    (:`LoopBody`
      (if (== (`.ID_17_7B6B61C64FC1EF1CFBC9F7A7BCA14F28` (break `/Game/RPG/RadarSystem/Structs/s_DynamicMarker` _arrayelement)) (`local.LocalID`))
        (`self.RemoveMarker` _arrayindex)))
    (:`Completed`
      (return))))

(fn `ScanWorldMarkers`
  (bind _outactors (`GameplayStatics.GetAllActorsWithInterface` "/Game/RPG/RadarSystem/Blueprints/BPI_Marker.BPI_Marker_C"))
  (for _array_element _outactors
    (bind (_id _markertype _movable_ _canbescanned_) (message `/Game/RPG/RadarSystem/Blueprints/BPI_Marker.GetMarkerData` _array_element))
    (if _canbescanned_
      (`self.AddActorMarker` _array_element)))
  (return))

(fn `UpdateDirections`
  (locals (LocalTraslation :type "Vector2D Structure") (LocalOnRadarSight :type Boolean :default false) (LocalDirection :type Name))
  (bind (_translation _clockwise_ _onradarsight_) (`self.ConvertRotationToTranslation` (`SceneComponent.K2_GetComponentRotation` (`self.PlayerCamera`)) (`KismetMathLibrary.MakeRotator` 0.0 0.0 (`KismetMathLibrary.Conv_IntToDouble` (`BlueprintMapLibrary.Map_Find` (`self.Directions`) (`local.LocalDirection`))))))
  (bind _keys (`BlueprintMapLibrary.Map_Keys` (`self.Directions`)))
  (for _array_element _keys
    (set `local.LocalDirection` _array_element)
    (set `local.LocalTraslation` _translation)
    (bind _output_get (set `local.LocalOnRadarSight` _onradarsight_))
    (`self.UpdateDirectionPosition` (`local.LocalDirection`) (`local.LocalTraslation`) _output_get))
  (return))

(fn `UpdateMarkerDistances`
  (params (`OnlyMovables?` :type Boolean))
  (locals (LocalCurrentLoopIndex :type Integer) (LocalDynamicMarker :type "/Game/RPG/RadarSystem/Structs/s_DynamicMarker Structure") (`LocalOnlyMovables?` :type Boolean))
  (set `local.LocalOnlyMovables?` `OnlyMovables?`)
  (bind (_arrayindex _arrayelement) (`/Engine/EditorBlueprintResources/StandardMacros.ReverseForEachLoop` (`self.Markers`))
    (:`LoopBody`
      (set `local.LocalCurrentLoopIndex` _arrayindex)
      (bind _output_get (set `local.LocalDynamicMarker` _arrayelement))
      (if (`.ShowDistanceFromPlayer?_8_A87F4C95411AEA2AB395BDA758FD5075` (break `/Game/RPG/RadarSystem/Structs/s_MarkerTypeData` (`.MarkerData_2_327873384C9A4B8B40B54EB079B777F8` (break `/Game/RPG/RadarSystem/Structs/s_DynamicMarker` _output_get))))
        (`/Engine/EditorBlueprintResources/StandardMacros.IsValid` (`.AttachedActor_6_584AF733497E0D1B9A2C08AB05C24118` (break `/Game/RPG/RadarSystem/Structs/s_DynamicMarker` (`local.LocalDynamicMarker`)))
          (:`Is Valid`
            (if (`local.LocalOnlyMovables?`)
              (if (`self.IsActorMoving?` (`.AttachedActor_6_584AF733497E0D1B9A2C08AB05C24118` (break `/Game/RPG/RadarSystem/Structs/s_DynamicMarker` (`local.LocalDynamicMarker`))))
                (`self.UpdateMarkerDistance` (`local.LocalCurrentLoopIndex`) (`/Game/RPG/RadarSystem/Blueprints/BPL_Radar.ConvertUnrealUnitsToMetric` (`self.Metric`) (`Actor.GetHorizontalDistanceTo` (`.AttachedActor_6_584AF733497E0D1B9A2C08AB05C24118` (break `/Game/RPG/RadarSystem/Structs/s_DynamicMarker` (`local.LocalDynamicMarker`))) (`self.Player`))) :!label _label))
              (else
                (goto _label))))
          (:`Is Not Valid`
            (`self.RemoveMarker` (`local.LocalCurrentLoopIndex`))))))
    (:`Completed`
      (return))))

(fn `UpdateMarkerElevationArrows`
  (params (`OnlyMovables?` :type Boolean))
  (locals (LocalCurrentLoopIndex :type Integer) (LocalDynamicMarker :type "/Game/RPG/RadarSystem/Structs/s_DynamicMarker Structure") (`LocalOnlyMovables?` :type Boolean))
  (bind (_up_ _hide_) (`self.CalculateMarkerArrow` (`.AttachedActor_6_584AF733497E0D1B9A2C08AB05C24118` (break `/Game/RPG/RadarSystem/Structs/s_DynamicMarker` (`local.LocalDynamicMarker`)))))
  (set `local.LocalOnlyMovables?` `OnlyMovables?`)
  (bind (_arrayindex _arrayelement) (`/Engine/EditorBlueprintResources/StandardMacros.ReverseForEachLoop` (`self.Markers`))
    (:`LoopBody`
      (set `local.LocalCurrentLoopIndex` _arrayindex)
      (bind _output_get (set `local.LocalDynamicMarker` _arrayelement))
      (if (`.ShowElevationArrow?_21_73364A6A4660514103329C957F2962A4` (break `/Game/RPG/RadarSystem/Structs/s_MarkerTypeData` (`.MarkerData_2_327873384C9A4B8B40B54EB079B777F8` (break `/Game/RPG/RadarSystem/Structs/s_DynamicMarker` _output_get))))
        (`/Engine/EditorBlueprintResources/StandardMacros.IsValid` (`.AttachedActor_6_584AF733497E0D1B9A2C08AB05C24118` (break `/Game/RPG/RadarSystem/Structs/s_DynamicMarker` (`local.LocalDynamicMarker`)))
          (:`Is Valid`
            (if (`local.LocalOnlyMovables?`)
              (if (`self.IsActorMoving?` (`.AttachedActor_6_584AF733497E0D1B9A2C08AB05C24118` (break `/Game/RPG/RadarSystem/Structs/s_DynamicMarker` (`local.LocalDynamicMarker`))))
                (`self.UpdateMarkerElevationArrow` (`local.LocalCurrentLoopIndex`) _up_ _hide_ :!label _label))
              (else
                (goto _label))))
          (:`Is Not Valid`
            (`self.RemoveMarker` (`local.LocalCurrentLoopIndex`))))))
    (:`Completed`
      (return))))

(fn `UpdateMarkerPositions`
  (params (`OnlyMovables?` :type Boolean))
  (locals (LocalTranslation :type "Vector2D Structure") (LocalClockWise :type Boolean :default false) (LocalOnRadarSight :type Boolean :default false) (LocalCurrentLoopIndex :type Integer) (LocalDynamicMarker :type "/Game/RPG/RadarSystem/Structs/s_DynamicMarker Structure") (`LocalOnlyMovables?` :type Boolean))
  (bind (_translation _clockwise_ _onradarsight_) (`self.ConvertRotationToTranslation` (`SceneComponent.K2_GetComponentRotation` (`self.PlayerCamera`)) (`KismetMathLibrary.FindLookAtRotation` (`Actor.K2_GetActorLocation` (`self.Player`)) (`Actor.K2_GetActorLocation` (`.AttachedActor_6_584AF733497E0D1B9A2C08AB05C24118` (break `/Game/RPG/RadarSystem/Structs/s_DynamicMarker` (`local.LocalDynamicMarker`)))))))
  (set `local.LocalOnlyMovables?` `OnlyMovables?`)
  (bind (_arrayindex _arrayelement) (`/Engine/EditorBlueprintResources/StandardMacros.ReverseForEachLoop` (`self.Markers`))
    (:`LoopBody`
      (set `local.LocalCurrentLoopIndex` _arrayindex)
      (bind _output_get (set `local.LocalDynamicMarker` _arrayelement))
      (`/Engine/EditorBlueprintResources/StandardMacros.IsValid` (`.AttachedActor_6_584AF733497E0D1B9A2C08AB05C24118` (break `/Game/RPG/RadarSystem/Structs/s_DynamicMarker` _output_get))
        (:`Is Valid`
          (if (`local.LocalOnlyMovables?`)
            (if (`self.IsActorMoving?` (`.AttachedActor_6_584AF733497E0D1B9A2C08AB05C24118` (break `/Game/RPG/RadarSystem/Structs/s_DynamicMarker` (`local.LocalDynamicMarker`))))
              (set `local.LocalTranslation` _translation :!label _label)
              (set `local.LocalClockWise` _clockwise_)
              (set `local.LocalOnRadarSight` _onradarsight_)
              (if (`.HideWhenOutOfSight?_19_BF03082D4F243FD0A887BC9B439B867A` (break `/Game/RPG/RadarSystem/Structs/s_MarkerTypeData` (`.MarkerData_2_327873384C9A4B8B40B54EB079B777F8` (break `/Game/RPG/RadarSystem/Structs/s_DynamicMarker` (`local.LocalDynamicMarker`)))))
                _
                (elif (not (`local.LocalOnRadarSight`))
                  (set `local.LocalTranslation` (`KismetMathLibrary.MakeVector2D` (`KismetMathLibrary.SelectFloat` (`self.MaxWidgetTranslation`) (* (`self.MaxWidgetTranslation`) -1.0) (`local.LocalClockWise`))))))
              (`self.UpdateMarkerPosition` (`local.LocalCurrentLoopIndex`) (`local.LocalTranslation`) (`local.LocalOnRadarSight`) (`.HideWhenOutOfSight?_19_BF03082D4F243FD0A887BC9B439B867A` (break `/Game/RPG/RadarSystem/Structs/s_MarkerTypeData` (`.MarkerData_2_327873384C9A4B8B40B54EB079B777F8` (break `/Game/RPG/RadarSystem/Structs/s_DynamicMarker` (`local.LocalDynamicMarker`)))))))
            (else
              (goto _label))))
        (:`Is Not Valid`
          (`self.RemoveMarker` (`local.LocalCurrentLoopIndex`)))))
    (:`Completed`
      (return))))

(fn `UpdateMarkers`
  (params (`OnlyMovables?` :type Boolean))
  (`self.UpdateMarkerPositions` `OnlyMovables?`)
  (`self.UpdateMarkerDistances` `OnlyMovables?`)
  (`self.UpdateMarkerElevationArrows` `OnlyMovables?`)
  (return))

(fn `UpdateRadar`
  (`self.UpdateDirections`)
  (`self.UpdateMarkers` false)
  (return))