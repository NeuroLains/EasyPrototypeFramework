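; BP_MsSphere is a floating NPC that starts a dialogue when the player character overlaps its collision sphere.
; Tick bobs the mesh around its starting height by a per-frame Z offset, not scaled by delta time.
; On overlap it passes its Dialogue asset and itself to BP_ThirdPersonCharacter's StartDialogueWithNPC.
; Dialogue participant functions supply name, icon and feminine gender, while condition, value and event handlers are stubs.
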(event `self.ReceiveBeginPlay`
  (bind (_returnvalue_x _returnvalue_y _returnvalue_z) (`KismetMathLibrary.BreakVector` (`SceneComponent.K2_GetComponentLocation` (`self.Sphere`))))
  ;[1 1 1] Move Sphere up down
  (set `self.InitialZValue` _returnvalue_z))

(event `self.ReceiveTick`
  (params (DeltaSeconds :type "Float (single-precision)"))
  (bind (_returnvalue_x _returnvalue_y _returnvalue_z) (`KismetMathLibrary.BreakVector` (`SceneComponent.K2_GetComponentLocation` (`self.Sphere`))))
  ;[1 1 1] Move Sphere up down
  (if (> (`KismetMathLibrary.Abs` (- _returnvalue_z (`self.InitialZValue`))) 50.0)
    (`/Engine/EditorBlueprintResources/StandardMacros.NegateFloat` (`self.ZVelocity`)
      (:`  `
        _)))
  (`SceneComponent.K2_AddWorldOffset` (`self.Sphere`) (`KismetMathLibrary.MakeVector` 0.0 0.0 (`self.ZVelocity`)) false false))

(event `self.CollisionSphere.OnComponentBeginOverlap`
  (params (OverlappedComponent :type "PrimitiveComponent Object Reference") (OtherActor :type "Actor Object Reference") (OtherComp :type "PrimitiveComponent Object Reference") (OtherBodyIndex :type Integer) (bFromSweep :type Boolean) (SweepResult :type "HitResult Structure (by ref)"))
  ;[1 0.4374 0.4474] Overlap with Player
  ;;[1 1 1] Cast to check if the overlap is with our player character
  (bind _asbp_third_person_character (cast `/Game/Dialogue/BP_ThirdPersonCharacter` OtherActor)
    (:`then`
      ;;[1 1 1] Start Dialogue between the Player and the NPC (MsSphere)
      (`/Game/Dialogue/BP_ThirdPersonCharacter.StartDialogueWithNPC` _asbp_third_person_character (`self.Dialogue`) self))
    (:`CastFailed`
      (`KismetSystemLibrary.PrintString` "BP_MsSphere Cast failed to ThirdPersonCharacter" true true (struct :`R` 1.0 :`A` 1.0) 5.0))))

(fn `CheckCondition`
  (params (Context :type "DlgContext Object Reference") (ConditionName :type Name))
  (returns (ReturnValue :type Boolean))
  (return false))

(fn `GetBoolValue`
  (params (ValueName :type Name))
  (returns (ReturnValue :type Boolean))
  (return false))

(fn `GetFloatValue`
  (params (ValueName :type Name))
  (returns (ReturnValue :type "Float (single-precision)"))
  (return 0.0))

(fn `GetIntValue`
  (params (ValueName :type Name))
  (returns (ReturnValue :type Integer))
  (return 0))

(fn `GetNameValue`
  (params (ValueName :type Name))
  (returns (ReturnValue :type Name))
  (return "None"))

(fn `GetParticipantDisplayName`
  (params (ActiveSpeaker :type Name))
  (returns (ReturnValue :type Text))
  (return (`self.DialogueParticipantDisplayName`)))

(fn `GetParticipantGender`
  (returns (ReturnValue :type "ETextGender Enum"))
  (return "Feminine"))

(fn `GetParticipantIcon`
  (params (ActiveSpeaker :type Name) (ActiveSpeakerState :type Name))
  (returns (ReturnValue :type "Texture2D Object Reference"))
  (return (`self.DialogueParticipantActiveIcon`)))

(fn `GetParticipantName`
  (returns (ReturnValue :type Name))
  (return (`self.DialogueParticipantName`)))

(fn `ModifyBoolValue`
  (params (ValueName :type Name) (bNewValue :type Boolean))
  (returns (ReturnValue :type Boolean))
  (return false))

(fn `ModifyFloatValue`
  (params (ValueName :type Name) (bDelta :type Boolean) (Value :type "Float (single-precision)"))
  (returns (ReturnValue :type Boolean))
  (return false))

(fn `ModifyIntValue`
  (params (ValueName :type Name) (bDelta :type Boolean) (Value :type Integer))
  (returns (ReturnValue :type Boolean))
  (return false))

(fn `ModifyNameValue`
  (params (ValueName :type Name) (NameValue :type Name))
  (returns (ReturnValue :type Boolean))
  (return false))

(fn `OnDialogueEvent`
  (params (Context :type "DlgContext Object Reference") (EventName :type Name))
  (returns (ReturnValue :type Boolean))
  (return false))

(fn `UserConstructionScript`)